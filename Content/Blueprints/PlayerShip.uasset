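; Player ship pawn that moves in the camera plane, fires bullets on a repeating timer and manages lives.
; Facing input rotates the ship and offsets the spring arm along an aspect-ratio-adjusted ellipse, which also sizes the spawned fog of war.
; Hits fracture the destructible hull and remove a HUD life, then destroy the actor or revive it with glowing temporary invulnerability.
; Lagged pursuit of the hit sphere drives a ghost and location-prediction point.
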(event OnComponentBeginOverlap(HitSphere)
  (params (OverlappedComponent :type Primitive%20Component%20Object%20Reference) (OtherActor :type Actor%20Object%20Reference) (OtherComp :type Primitive%20Component%20Object%20Reference) (OtherBodyIndex :type Integer) (bFromSweep :type Boolean) (SweepResult :type Hit%20Result%20Structure%20%28by%20ref%29))
  (bind _hull (Variables|Default|GetHull))
  (Utilities|Unless (Variables|Default|GetInvulnerable))
  (Utilities|WhenAlive)
  (Class|DestructibleComponent|ApplyRadiusDamage _hull 2.0 (Transformation|GetWorldLocation _hull) 33.0 33333.332031 true)
  (CallFunction|DecrementLives)
  (Variables|Default|SetAlive false)
  (Utilities|FlowControl|Delay 2.0)
  (Class|DestructibleComponent|SetDestructibleMesh (Variables|Default|GetHull) "/Game/Meshes/PlayerShipHull.PlayerShipHull")
  (if (< (Variables|Default|GetLives) 0)
    (Actor|DestroyActor)
    (else
      (Variables|Default|SetAlive true)
      (Variables|Default|SetInvulnerable true)
      (bind _emissivestrength (Timeline|InvulnerabilityTimeline PlayFromStart)
        (:Update
          (Rendering|Material|SetScalarParameterValue (Variables|Default|GetShipMaterial) "EmissiveStrength" _emissivestrength :!class /Script/Engine.MaterialInstanceDynamic))
        (:Finished
          (Variables|Default|SetInvulnerable false))))))

(event Custom|Shoot
  (Utilities|WhenAlive)
  (CallFunction|SpawnBullet))

(event Custom|StartShooting
  (bind _returnvalue (Utilities|Time|SetTimerbyEvent (delegate Custom|Shoot) 0.1667 true))
  (CallFunction|Shoot))

(event Custom|StopShooting
  (Utilities|Time|ClearandInvalidateTimerbyHandle (stale Custom|StartShooting _returnvalue)))

(event EventBeginPlay
  (Class|ZJoyBlueprintFunctionLibrary|MaintainMinorAxisFov self)
  (bind _asplayer_controller (Utilities|Casting|CastToPlayerController (Pawn|GetController)))
  (CallFunction|SpawnHudLives _asplayer_controller)
  (CallFunction|SpawnFogOfWar _asplayer_controller))

(event EventTick
  (params (DeltaSeconds :type Float%20%28single-precision%29))
  (Utilities|WhenAlive)
  (CallFunction|MoveForward DeltaSeconds)
  (CallFunction|FaceFacingInput)
  (Class|ZJoyBlueprintFunctionLibrary|MaintainMinorAxisFov self)
  (CallFunction|MatchFogOfWartoAspectRatio)
  (CallFunction|Pursue (Transformation|GetWorldLocation (Variables|Default|GetHitSphere)) (Variables|Default|GetHitSphereGhost) (Variables|Default|GetHitSphereGhostLag))
  (CallFunction|Pursue (/ (+ (Transformation|GetWorldLocation (Variables|Default|GetHitSphereGhost)) (Transformation|GetWorldLocation (Variables|Default|GetSpringArm))) 2.0) (Variables|Default|GetLocationPrediction) 0.5))

(event Input|AxisEvents|InputAxisMoveUp
  (params (AxisValue :type Float%20%28single-precision%29))
  (Utilities|WhenAlive)
  (Pawn|Input|AddMovementInput (Math|Vector|GetUpVector (Variables|Default|GetCamera)) AxisValue false))

(event Input|AxisEvents|InputAxisMoveRight
  (params (AxisValue :type Float%20%28single-precision%29))
  (Utilities|WhenAlive)
  (Pawn|Input|AddMovementInput (Math|Vector|GetRightVector (Variables|Default|GetCamera)) AxisValue false))

(fn ConstructionScript
  (Variables|Default|SetConstructedDistanceBetweenShipAndSpringArm (Math|Vector|Distance2D(Vector) (Transformation|GetWorldLocation (Variables|Default|GetSpringArm)) (Transformation|GetWorldLocation (Variables|Default|GetHull))))
  (Variables|Default|SetConstructedSpringArmLength (Variables|/Script/Engine.SpringArmComponent|GetTargetArmLength (Variables|Default|GetSpringArm)))
  (bind _returnvalue (Rendering|Material|CreateDynamicMaterialInstance (Variables|Default|GetHull) 0 "/Game/Materials/Player.Player" "None" :!class /Script/Engine.PrimitiveComponent))
  (Variables|Default|SetShipMaterial _returnvalue)
  (Variables|Default|SetConstructedSpeedMultiplierCubeScaleZ (.z (Transformation|GetWorldScale (Variables|Default|GetSpeedMutiplierCube)))))

(fn SetFacingInputRight
  (params (Right :type Float%20%28single-precision%29) (WorldRight :type Vector))
  (bind _returnvalue (Math|Rotator|MakeRotfromY WorldRight))
  (Variables|Default|SetFacingInput (Math|Vector|RotateVector (Math|Vector|MakeVector (.x (Math|Vector|RotateVector (Variables|Default|GetFacingInput) (Class|KismetMathLibrary|NegateRotator _returnvalue))) Right (.z (Math|Vector|RotateVector (Variables|Default|GetFacingInput) (Class|KismetMathLibrary|NegateRotator _returnvalue)))) _returnvalue)))

(fn SetFacingInputUp
  (params (Up :type Float%20%28single-precision%29) (WorldUp :type Vector))
  (bind _returnvalue (Math|Rotator|MakeRotfromZ WorldUp))
  (Variables|Default|SetFacingInput (Math|Vector|RotateVector (Math|Vector|MakeVector (.x (Math|Vector|RotateVector (Variables|Default|GetFacingInput) (Class|KismetMathLibrary|NegateRotator _returnvalue))) (.y (Math|Vector|RotateVector (Variables|Default|GetFacingInput) (Class|KismetMathLibrary|NegateRotator _returnvalue))) Up) _returnvalue)))

(fn SpringArmDistancewhenFacing
  (params (Point :type Vector%202D%20Structure))
  (bind _constructeddistancebetweenshipandspringarm (Variables|Default|GetConstructedDistanceBetweenShipAndSpringArm))
  (bind _semiaxeslengths (CallFunction|SemiAxesLengthsatViewPortAspectRatio _constructeddistancebetweenshipandspringarm))
  (bind (_x _y) (Math|Vector2D|BreakVector2D _semiaxeslengths))
  (return (* (Math|Float|Clamp(Float) (Math|Float|Square (Variables|Default|GetFacingInputMagnitude))) (Math|Vector2D|Vector2DLength (Class|ZJoyBlueprintFunctionLibrary|EllipseLineIntersection Point _x _y)))))

(fn SpawnBullet
  (bind _returnvalue (Transformation|GetActorRotation))
  (Game|SpawnActorfromClass "/Game/Blueprints/PlayerBullet.PlayerBullet_C" (Math|Transform|MakeTransform (+ (Transformation|GetActorLocation) (Math|Vector|RotateVector "100.000000, 0, 0" _returnvalue)) _returnvalue) "Undefined" 0 0.0 0 self))

(fn MatchSpringArmLocationtoFacingVector
  (params (Point :type Vector))
  (bind _returnvalue (CallFunction|RotateWorldtoCamera Point))
  (Transformation|SetRelativeLocation (Variables|Default|GetSpringArm) (Math|Vector|MakeVector (CallFunction|SpringArmDistancewhenFacing (Math|Vector2D|MakeVector2D (.y _returnvalue) (.z _returnvalue))) 0.0 0.0) false false))

(fn GetFacingVector
  (bind _returnvalue (Class|Pawn|GetLastMovementInputVector))
  (bind _facinginput (Variables|Default|GetFacingInput))
  (bind _returnvalue_2 (Math|Vector|VectorIsNearlyZero _facinginput))
  (bind _returnvalue_3 (select _returnvalue_2 _returnvalue _facinginput))
  (return (select (Math|Vector|VectorIsNearlyZero _returnvalue_3) (Transformation|GetActorForwardVector) _returnvalue_3)))

(fn MoveForward
  (params (DeltaSeconds :type Float%20%28single-precision%29))
  (bind _returnvalue (Class|Pawn|ConsumeMovementInputVector))
  (Transformation|AddActorWorldOffset (* (Math|Vector|ClampVectorSize _returnvalue 0.0 1.0) (* DeltaSeconds (* (Variables|Default|GetSpeed) (Variables|Default|GetSpeedMultiplier)))) true))

(fn SpawnHudLives
  (params (PlayerController :type Player%20Controller%20Object%20Reference))
  (for _index (range 0 (- (Variables|Default|GetLives) 1))
    (bind _returnvalue (Game|SpawnActorfromClass "/Game/Blueprints/PlayerShipHudLife.PlayerShipHudLife_C" (CallFunction|UnitTransform) "Undefined" 0 1e+01 (Math|Vector2D|MakeVector2D (+ (* _index 0.03) 0.03) 0.03) PlayerController 0))
    (Utilities|Array|Add (Variables|Default|GetHudLives) _returnvalue)))

(fn SpawnFogOfWar
  (params (PlayerController :type Player%20Controller%20Object%20Reference))
  (bind _fogofwarunitradius (Variables|Default|GetFogOfWarUnitRadius))
  (bind _returnvalue (Game|SpawnActorfromClass "/Game/Blueprints/FogOfWar.FogOfWar_C" (CallFunction|UnitTransform) "Undefined" 0 (Math|Vector2D|MakeVector2D _fogofwarunitradius _fogofwarunitradius) 1e+01 "(X=0.500000,Y=0.500000)" PlayerController 0))
  (Variables|Default|SetFogOfWar _returnvalue))

(fn MatchFogOfWartoAspectRatio
  (Default|SetAxesLengths (Variables|Default|GetFogOfWar) (CallFunction|SemiAxesLengthsatViewPortAspectRatio (Variables|Default|GetFogOfWarUnitRadius))))

(fn SemiAxesLengthsatViewPortAspectRatio
  (params (UnitRadius :type Float%20%28single-precision%29))
  (bind _aspectratio (CallFunction|GetViewportAspectRatio))
  (return (Math|Vector2D|MakeVector2D (* (Math|Float|Clamp(Float) _aspectratio 1.0 1.33) UnitRadius) (* (Math|Float|Clamp(Float) (/ 1.0 _aspectratio) 1.0 1.33) UnitRadius))))

(fn FaceFacingInput
  (bind _facinginput (Variables|Default|GetFacingInput))
  (Transformation|SetActorRotation (Math|Rotator|FindLookatRotation (Math|Vector|MakeVector 0.0 0.0 0.0) _facinginput))
  (CallFunction|MatchSpringArmLocationtoFacingVector _facinginput))

(fn RotateWorldtoCamera
  (params (A :type Vector))
  (return (Math|Vector|RotateVector A (Class|KismetMathLibrary|NegateRotator (Transformation|GetWorldRotation (Variables|Default|GetCamera))))))

(fn DecrementLives
  (bind _hudlives (Variables|Default|GetHudLives))
  (if (> (Variables|Default|GetLives) 0)
    (Actor|DestroyActor (Utilities|GetLast _hudlives))
    (Utilities|RemoveLast _hudlives))
  (Math|Integer|DecrementInt (Variables|Default|GetLives)))

(fn SetSpeedMultiplier
  (params (Multiplier :type Float%20%28single-precision%29))
  (bind _speedmutipliercube (Variables|Default|GetSpeedMutiplierCube))
  (bind _returnvalue (Transformation|GetWorldScale _speedmutipliercube))
  (bind _output_get (Variables|Default|SetSpeedMultiplier Multiplier))
  (Transformation|SetWorldScale3D _speedmutipliercube (Math|Vector|MakeVector (.x _returnvalue) (.y _returnvalue) (* _output_get (Variables|Default|GetConstructedSpeedMultiplierCubeScaleZ)))))

(fn Pursue
  (params (PurusedLocation :type Vector) (Pursuer :type Scene%20Component%20Object%20Reference) (Lag :type Float%20%28single-precision%29))
  (Transformation|SetWorldLocation Pursuer (CallFunction|PursuitLocation PurusedLocation (Transformation|GetWorldLocation Pursuer) (Utilities|Time|GetWorldDeltaSeconds) Lag) false false))