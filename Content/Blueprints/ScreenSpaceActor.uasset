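; An actor that stays pinned to a point on the player's screen while existing in world space.
; Each Tick it deprojects ScreenPosition, scaled by the viewport size, into the world and pushes it along the view direction by DirectionOffset.
; It also copies the player camera manager's rotation, so its orientation matches the camera.
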(event EventBeginPlay)

(event Collision|EventActorBeginOverlap
  (params (OtherActor :type Actor%20Object%20Reference)))

(event EventTick
  (params (DeltaSeconds :type Float%20%28single-precision%29))
  (Transformation|SetActorLocation (CallFunction|ScreenPositioninWorldSpace) false false)
  (Transformation|SetActorRotation (CallFunction|PlayerCameraRotation)))

(fn ConstructionScript)

(fn ScreenPositioninWorldSpace
  (bind _returnvalue (Viewport|GetViewportSize))
  (bind _screenposition (Variables|Default|GetScreenPosition))
  (bind _playercontroller (Variables|Default|GetPlayerController))
  (bind _returnvalue_2 (* _returnvalue _screenposition))
  (bind (_worldposition _worlddirection) (Class|GameplayStatics|DeprojectScreentoWorld _playercontroller _returnvalue_2))
  (return (+ _worldposition (* _worlddirection (Variables|Default|GetDirectionOffset)))))

(fn PlayerCameraRotation
  (return (Camera|GetCameraRotation (Variables|/Script/Engine.PlayerController|GetPlayerCameraManager (Variables|Default|GetPlayerController)))))