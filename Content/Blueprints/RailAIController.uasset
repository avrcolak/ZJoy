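; AI controller that moves its possessed pawn along a spline rail once, then unpossesses and destroys itself.
; The FollowRail timeline is rescaled to the spline's duration and drives a swept move along it each update.
; Float curves injected in the construction script set a yaw offset from the initial heading and a blend toward facing the target's HitSphere, with interpolated rotation.
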(event EventPossess
  (params (PossessedPawn :type Pawn%20Object%20Reference))
  (Utilities|IsValid PossessedPawn
    (:Is%20Valid
      (Variables|Default|SetInitialYaw (.yaw (Transformation|GetActorRotation PossessedPawn)))
      (Utilities|FlowControl|Sequence
        (:then_0
          (Components|Timeline|SetPlayRate (Variables|Default|GetFollowRail) (/ 1.0 (CallFunction|GetSplineDuration))))
        (:then_1
          (bind (_direction _yaw _facetarget) (Timeline|FollowRail PlayFromStart)
            (:Update
              (bind _yawtofacetarget (CallFunction|YawtoFaceTarget))
              (Transformation|SetActorLocationAndRotation (Pawn|GetControlledPawn) (Spline|GetLocationatTime (Variables|/Game/Blueprints/Splines/SplineActor.SplineActor_C|GetSpline (Variables|Default|GetSplineActor)) (* (Components|Timeline|GetPlaybackPosition (Variables|Default|GetFollowRail)) (CallFunction|GetSplineDuration)) "World" false) (CallFunction|RInterpPawnRotationto _yaw _yawtofacetarget _facetarget) true))
            (:Finished
              (Pawn|UnPossess))))))))

(event EventUnPossess
  (params (UnpossessedPawn :type Pawn%20Object%20Reference))
  (Actor|DestroyActor))

(fn ConstructionScript
  (Class|TimelineComponent|SetFloatCurve (Variables|Default|GetFollowRail) (Variables|Default|GetYaw) "Yaw")
  (Class|TimelineComponent|SetFloatCurve (Variables|Default|GetFollowRail) (Variables|Default|GetFaceTarget) "FaceTarget"))

(fn RInterpPawnRotationto
  (params (Yaw :type Float%20%28single-precision%29) (YawToFaceTarget :type Float%20%28single-precision%29) (FaceTarget :type Float%20%28single-precision%29))
  (return (Math|Interpolation|RInterpTo (Transformation|GetActorRotation (Pawn|GetControlledPawn)) (Math|Rotator|MakeRotator 0.0 0.0 (Math|Float|Lerp (+ (Variables|Default|GetInitialYaw) Yaw) YawToFaceTarget FaceTarget)) (Utilities|Time|GetWorldDeltaSeconds) 3.333333)))

(fn YawtoFaceTarget
  (Utilities|IsValid (Variables|Default|GetTarget)
    (:Is%20Valid
      (return (.yaw (Math|Rotator|FindLookatRotation (Transformation|GetActorLocation (Pawn|GetControlledPawn)) (Transformation|GetWorldLocation (Variables|/Game/Blueprints/PlayerShip.PlayerShip_C|GetHitSphere (Variables|Default|GetTarget)))))))
    (:Is%20Not%20Valid
      (return (Variables|Default|GetInitialYaw)))))

(fn GetSplineDuration
  (return (Variables|/Script/Engine.SplineComponent|GetDuration (Variables|/Game/Blueprints/Splines/SplineActor.SplineActor_C|GetSpline (Variables|Default|GetSplineActor)))))