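; Player controller that turns mouse or axis input into PlayerShip facing, speed, shooting and camera roll.
; Tick switches to mouse aim when the cursor moves (axis input switches back), then feeds the ship a camera-relative direction, magnitude and cycled speed multiplier.
; It keeps the score on a spawned ScreenSpaceText actor and, on unpossessing a ship, possesses a new spectator pawn at its camera.
; Input-mode hacks work around focus and cursor issues.
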(event EventBeginPlay
  (bind _returnvalue (Game|SpawnActorfromClass "/Game/Blueprints/ScreenSpaceText.ScreenSpaceText_C" (CallFunction|UnitTransform) "Undefined" 0 9.0 "(X=0.990000,Y=0.010000)" self 0))
  (bind _output_get (Variables|Default|SetScoreDisplay _returnvalue))
  (Rendering|Components|TextRender|SetHorizontalAlignment (Variables|/Game/Blueprints/ScreenSpaceText.ScreenSpaceText_C|GetTextRender _output_get) "EHTA_Right")
  (CallFunction|UpdateScoreDisplay))

(event EventTick
  (params (DeltaSeconds :type Float%20%28single-precision%29))
  (bind (_returnvalue _mouseposition) (CallFunction|GetNormalizedMousePositionfromViewportCenter))
  (bind (_direction _magnitude) (CallFunction|FacingVector))
  (bind (_x _y) (Math|Vector2D|BreakVector2D _direction))
  (Utilities|When _returnvalue)
  (bind _output_get (Variables|Default|SetMousePosition _mouseposition))
  (if (Class|KismetMathLibrary|IsNearlyZero2D (- _output_get (Variables|Default|GetPreviousMousePosition)) 0.0001)
    _
    (else
      (CallFunction|StartUsingMouse)))
  (bind _asplayership (Utilities|WhenControlledPawnIsPlayerShip))
  (CallFunction|SetPlayerShipFacing _asplayership _x _y _magnitude)
  (CallFunction|SetPlayerShipSpeedMultiplier _asplayership)
  (Variables|Default|SetPreviousMousePosition (Variables|Default|GetMousePosition)))

(event EventUnPossess
  (params (UnpossessedPawn :type Pawn%20Object%20Reference))
  (bind _asplayer_ship (Utilities|Casting|CastToPlayerShip UnpossessedPawn))
  (bind _returnvalue (Game|SpawnActorfromClass "/Script/Engine.SpectatorPawn" (Transformation|GetWorldTransform (Actor|GetComponentbyClass _asplayer_ship "/Script/Engine.CameraComponent")) "Undefined" 0 0))
  (Pawn|Possess _returnvalue))

(event Input|ActionEvents|InputActionShoot
  (params (Key :type Key%20Structure))
  (:Pressed
    (bind _asplayership (Utilities|WhenControlledPawnIsPlayerShip))
    (Default|StartShooting _asplayership))
  (:Released
    (bind _asplayership_2 (Utilities|WhenControlledPawnIsPlayerShip))
    (Default|StopShooting _asplayership_2)))

(event Input|ActionEvents|InputActionCycleSpeed
  (params (Key :type Key%20Structure))
  (:Pressed
    (Math|Float|DecrementFloat (Variables|Default|GetSpeedMultiplier)))
  (:Released
    (Utilities|When (<= (Variables|Default|GetSpeedMultiplier) 1.0))
    (Variables|Default|SetSpeedMultiplier 4.0)))

(event Input|AxisEvents|InputAxisRotateCameraRight
  (params (AxisValue :type Float%20%28single-precision%29))
  (bind _asplayership (Utilities|WhenControlledPawnIsPlayerShip))
  (Transformation|AddLocalRotation (Variables|/Game/Blueprints/PlayerShip.PlayerShip_C|GetCamera _asplayership) (Math|Rotator|MakeRotator (* (Utilities|Time|GetWorldDeltaSeconds) (* AxisValue (Variables|Default|GetRotationSpeed))) 0.0 0.0) false false))

(event Input|AxisEvents|InputAxisFaceUp
  (params (AxisValue :type Float%20%28single-precision%29))
  (bind _output_get (Variables|Default|SetFaceUp AxisValue))
  (Utilities|Unless (Math|Float|NearlyEqual(Float) _output_get 0.0 1e-06))
  (CallFunction|StopUsingMouse))

(event Input|AxisEvents|InputAxisFaceRight
  (params (AxisValue :type Float%20%28single-precision%29))
  (bind _output_get (Variables|Default|SetFaceRight AxisValue))
  (Utilities|Unless (Math|Float|NearlyEqual(Float) _output_get 0.0 1e-06))
  (CallFunction|StopUsingMouse))

(event Input|KeyboardEvents|Escape
  (params (Key :type Key%20Structure))
  (:Pressed
    (Game|QuitGame self "Quit" false)))

(event Input|MouseEvents|LeftMouseButton
  (params (Key :type Key%20Structure))
  ;[1 1 1] Hack to prevent losing focus on click
  (:Released
    (Input|SetInputModeGameandUI self 0 "LockAlways" false)))

(fn ConstructionScript)

(fn IncrementScore
  (params (Amount :type Integer))
  (Variables|Default|SetScore (+ Amount (Variables|Default|GetScore)))
  (CallFunction|UpdateScoreDisplay))

(fn SetPlayerShipFacing
  (params (ZPawn :type Player%20Ship%20Object%20Reference) (Right :type Float%20%28single-precision%29) (Up :type Float%20%28single-precision%29) (Magnitude :type Float%20%28single-precision%29))
  (bind _camera (Variables|/Game/Blueprints/PlayerShip.PlayerShip_C|GetCamera ZPawn))
  (Utilities|When (Variables|/Game/Blueprints/PlayerShip.PlayerShip_C|GetAlive ZPawn))
  (Utilities|Unless (Class|KismetMathLibrary|IsNearlyZero2D (Math|Vector2D|MakeVector2D Right Up) 0.0001))
  (Default|SetFacingInputRight ZPawn Right (Math|Vector|GetRightVector _camera))
  (Default|SetFacingInputUp ZPawn Up (Math|Vector|GetUpVector _camera))
  (Variables|/Game/Blueprints/PlayerShip.PlayerShip_C|SetFacingInputMagnitude ZPawn Magnitude))

(fn GetNormalizedMousePositionfromViewportCenter
  (bind (_locationx _locationy _returnvalue) (Game|Player|GetMousePosition))
  (bind _returnvalue_2 (Viewport|GetViewportSize))
  (bind _returnvalue_3 (* _returnvalue_2 0.5))
  (bind _returnvalue_4 (Math|Vector2D|MakeVector2D _locationx _locationy))
  (bind _y (Math|Vector2D|BreakVector2D _returnvalue_2))
  (bind _returnvalue_5 (- _returnvalue_4 _returnvalue_3))
  (bind _returnvalue_6 (/ _returnvalue_5 _y))
  (bind _returnvalue_7 (* _returnvalue_6 2.0))
  (return _returnvalue (Math|Vector2D|MakeVector2D (.x _returnvalue_7) (.y _returnvalue_7))))

(fn StopUsingMouse
  (Variables|Default|SetPlayerUsingMouse false)
  (Variables|Default|SetbShowMouseCursor false)
  (Input|SetInputModeGameandUI self 0 "LockAlways" false) ; Hack to ensure mouse cursor gets hidden
)

(fn StartUsingMouse
  (Variables|Default|SetPlayerUsingMouse true)
  (Variables|Default|SetbShowMouseCursor true))

(fn UpdateScoreDisplay
  (Default|SetText (Variables|Default|GetScoreDisplay) (Utilities|Text|ToText(Integer) (Variables|Default|GetScore))))

(fn FacingVector
  (bind _returnvalue (Class|KismetMathLibrary|Vector2DZero))
  (bind _mouseposition (Variables|Default|GetMousePosition))
  (bind _faceright (Variables|Default|GetFaceRight))
  (bind _faceup (Variables|Default|GetFaceUp))
  (bind _playerusingmouse (Variables|Default|GetPlayerUsingMouse))
  (bind _returnvalue_2 (Math|Vector2D|MakeVector2D _faceright _faceup))
  (bind _returnvalue_3 (* (.y _mouseposition) -1.0))
  (bind _returnvalue_4 (Class|KismetMathLibrary|VSize2DSquared _returnvalue_2))
  (bind _returnvalue_5 (Math|Vector2D|MakeVector2D (.x _mouseposition) _returnvalue_3))
  (bind _returnvalue_6 (< _returnvalue_4 0.025))
  (bind _returnvalue_7 (select _returnvalue_6 _returnvalue _returnvalue_2))
  (bind _returnvalue_8 (select _playerusingmouse _returnvalue_5 _returnvalue_7))
  (return (Math|Vector2D|Normalize2D _returnvalue_8) (Math|Vector2D|Vector2DLength _returnvalue_8)))

(fn SetPlayerShipSpeedMultiplier
  (params (ZPawn :type Player%20Ship%20Object%20Reference))
  (Default|SetSpeedMultiplier ZPawn (Variables|Default|GetSpeedMultiplier)))