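; Player ship pawn for a twin-stick shooter, with camera-relative movement and facing, timer-driven fire, HUD lives and fog of war.
; Tick moves and rotates the ship, sliding the spring arm along an aspect-ratio-adjusted ellipse and resizing the fog to match.
; Hits fracture the destructible mesh and cost a life, restoring the ship after a delay or destroying it when none remain.
; A WhenAlive macro gates gameplay events.
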(event OnComponentBeginOverlap(HitSphere)
  (params (OverlappedComponent :type Primitive%20Component%20Object%20Reference) (OtherActor :type Actor%20Object%20Reference) (OtherComp :type Primitive%20Component%20Object%20Reference) (OtherBodyIndex :type Integer) (bFromSweep :type Boolean) (SweepResult :type Hit%20Result%20Structure%20%28by%20ref%29))
  (bind _hudlives (Variables|Default|GetHudLives))
  (Utilities|WhenAlive)
  (Class|DestructibleComponent|ApplyRadiusDamage (Variables|Default|GetShip) 2.0 (Transformation|GetActorLocation) 1e+02 0.0 true)
  (Actor|DestroyActor (Utilities|GetLast _hudlives))
  (Utilities|RemoveLast _hudlives)
  (Variables|Default|SetAlive false)
  (Math|Integer|DecrementInt (Variables|Default|GetLives)))

(event OnComponentFracture(Ship)
  (params (HitPoint :type Vector%20%28by%20ref%29 :default "0, 0, 0") (HitDirection :type Vector%20%28by%20ref%29 :default "0, 0, 0"))
  (Physics|AddRadialForce (Variables|Default|GetShip) HitPoint 1e+02 333333.0 "RIF_Constant" true)
  (Utilities|FlowControl|Delay 2.0)
  (Class|DestructibleComponent|SetDestructibleMesh (Variables|Default|GetShip) "/Game/Meshes/Pawn.Pawn")
  (if (<= (Variables|Default|GetLives) 0)
    (Actor|DestroyActor)
    (else
      (Variables|Default|SetAlive true))))

(event Custom|Shoot
  (Utilities|WhenAlive)
  (CallFunction|SpawnBullet))

(event EventBeginPlay
  (Class|ZJoyBlueprintFunctionLibrary|MaintainMinorAxisFov self)
  (bind _asplayer_controller (Utilities|Casting|CastToPlayerController (Pawn|GetController)))
  (CallFunction|SpawnHudLives _asplayer_controller)
  (CallFunction|SpawnFogOfWar _asplayer_controller))

(event EventTick
  (params (DeltaSeconds :type Float%20%28single-precision%29))
  (Utilities|WhenAlive)
  (CallFunction|MoveForward DeltaSeconds)
  (CallFunction|FaceFacingInput)
  (Class|ZJoyBlueprintFunctionLibrary|MaintainMinorAxisFov self)
  (CallFunction|MatchFogOfWartoAspectRatio))

(event Input|ActionEvents|InputActionShoot
  (params (Key :type Key%20Structure))
  (:Pressed
    (bind _returnvalue (Utilities|Time|SetTimerbyEvent (delegate Custom|Shoot) 0.1667 true)))
  (:Released
    (Utilities|Time|ClearandInvalidateTimerbyHandle _returnvalue)))

(event Input|AxisEvents|InputAxisMoveUp
  (params (AxisValue :type Float%20%28single-precision%29))
  (Utilities|WhenAlive)
  (Pawn|Input|AddMovementInput (Math|Vector|GetUpVector (Variables|Default|GetCamera)) AxisValue false))

(event Input|AxisEvents|InputAxisMoveRight
  (params (AxisValue :type Float%20%28single-precision%29))
  (Utilities|WhenAlive)
  (Pawn|Input|AddMovementInput (Math|Vector|GetRightVector (Variables|Default|GetCamera)) AxisValue false))

(event Input|AxisEvents|InputAxisFaceUp
  (params (AxisValue :type Float%20%28single-precision%29))
  (Utilities|WhenAlive)
  (CallFunction|SetFacingInputUp AxisValue (Math|Vector|GetUpVector (Variables|Default|GetCamera))))

(event Input|AxisEvents|InputAxisFaceRight
  (params (AxisValue :type Float%20%28single-precision%29))
  (Utilities|WhenAlive)
  (CallFunction|SetFacingInputRight AxisValue (Math|Vector|GetRightVector (Variables|Default|GetCamera))))

(event Input|KeyboardEvents|T
  (params (Key :type Key%20Structure))
  (:Pressed
    (bind _isa (Utilities|FlowControl|FlipFlop)
      (:A
        _)
      (:B
        _))
    (Transformation|SetAbsolute (Variables|Default|GetCamera) false _isa false)))

(fn ConstructionScript
  (Variables|Default|SetConstructedDistanceBetweenShipAndSpringArm (Math|Vector|Distance2D(Vector) (Transformation|GetWorldLocation (Variables|Default|GetSpringArm)) (Transformation|GetWorldLocation (Variables|Default|GetShip))))
  (Variables|Default|SetConstructedSpringArmLength (Variables|/Script/Engine.SpringArmComponent|GetTargetArmLength (Variables|Default|GetSpringArm))))

(fn SetFacingInputRight
  (params (Right :type Float%20%28single-precision%29) (WorldRight :type Vector))
  (bind _returnvalue (Math|Rotator|MakeRotfromY WorldRight))
  (Variables|Default|SetFacingInput (Math|Vector|RotateVector (Math|Vector|MakeVector (.x (Math|Vector|RotateVector (Variables|Default|GetFacingInput) (Class|KismetMathLibrary|NegateRotator _returnvalue))) Right (.z (Math|Vector|RotateVector (Variables|Default|GetFacingInput) (Class|KismetMathLibrary|NegateRotator _returnvalue)))) _returnvalue)))

(fn SetFacingInputUp
  (params (Up :type Float%20%28single-precision%29) (WorldUp :type Vector))
  (bind _returnvalue (Math|Rotator|MakeRotfromZ WorldUp))
  (Variables|Default|SetFacingInput (Math|Vector|RotateVector (Math|Vector|MakeVector (.x (Math|Vector|RotateVector (Variables|Default|GetFacingInput) (Class|KismetMathLibrary|NegateRotator _returnvalue))) (.y (Math|Vector|RotateVector (Variables|Default|GetFacingInput) (Class|KismetMathLibrary|NegateRotator _returnvalue))) Up) _returnvalue)))

(fn SpringArmDistancewhenFacing
  (params (Point :type Vector%202D%20Structure))
  (bind _constructeddistancebetweenshipandspringarm (Variables|Default|GetConstructedDistanceBetweenShipAndSpringArm))
  (bind _semiaxeslengths (CallFunction|SemiAxesLengthsatViewPortAspectRatio _constructeddistancebetweenshipandspringarm))
  (bind (_x _y) (Math|Vector2D|BreakVector2D _semiaxeslengths))
  (return (Math|Vector2D|Vector2DLength (Class|ZJoyBlueprintFunctionLibrary|EllipseLineIntersection Point _x _y))))

(fn SpawnBullet
  (bind _returnvalue (Transformation|GetActorRotation))
  (Game|SpawnActorfromClass "/Game/Blueprints/ZPawnBullet.ZPawnBullet_C" (Math|Transform|MakeTransform (+ (Transformation|GetActorLocation) (Math|Vector|RotateVector "1.000000, 0, 0" _returnvalue)) _returnvalue) "Undefined" 0 0.0 0 self))

(fn MatchSpringArmLocationtoFacingVector
  (params (Point :type Vector%202D%20Structure))
  (Transformation|SetRelativeLocation (Variables|Default|GetSpringArm) (Math|Vector|MakeVector (CallFunction|SpringArmDistancewhenFacing Point) 0.0 0.0) false false))

(fn GetFacingVector
  (bind _returnvalue (Class|Pawn|GetLastMovementInputVector))
  (bind _facinginput (Variables|Default|GetFacingInput))
  (bind _returnvalue_2 (Math|Vector|VectorIsNearlyZero _facinginput))
  (bind _returnvalue_3 (select _returnvalue_2 _returnvalue _facinginput))
  (return (select (Math|Vector|VectorIsNearlyZero _returnvalue_3) (Transformation|GetActorForwardVector) _returnvalue_3)))

(fn MoveForward
  (params (DeltaSeconds :type Float%20%28single-precision%29))
  (bind _returnvalue (Class|Pawn|ConsumeMovementInputVector))
  (Transformation|AddActorWorldOffset (* _returnvalue (* DeltaSeconds (Variables|Default|GetSpeed))) true))

(fn SpawnHudLives
  (params (PlayerController :type Player%20Controller%20Object%20Reference))
  (for _index (range 0 (- (Variables|Default|GetLives) 1))
    (bind _returnvalue (Game|SpawnActorfromClass "/Game/Blueprints/ZPawnHudLife.ZPawnHudLife_C" (CallFunction|UnitTransform) "Undefined" 0 1e+01 (Math|Vector2D|MakeVector2D (+ (* _index 0.03) 0.03) 0.03) PlayerController 0))
    (Utilities|Array|Add (Variables|Default|GetHudLives) _returnvalue)))

(fn SpawnFogOfWar
  (params (PlayerController :type Player%20Controller%20Object%20Reference))
  (bind _unitfogofwarradius (Variables|Default|GetUnitFogOfWarRadius))
  (bind _returnvalue (Game|SpawnActorfromClass "/Game/Blueprints/FogOfWar.FogOfWar_C" (CallFunction|UnitTransform) "Undefined" 0 (Math|Vector2D|MakeVector2D _unitfogofwarradius _unitfogofwarradius) 1e+01 "(X=0.500000,Y=0.500000)" PlayerController 0))
  (Variables|Default|SetFogOfWar _returnvalue))

(fn MatchFogOfWartoAspectRatio
  (Default|SetAxesLengths (Variables|Default|GetFogOfWar) (CallFunction|SemiAxesLengthsatViewPortAspectRatio (Variables|Default|GetUnitFogOfWarRadius))))

(fn SemiAxesLengthsatViewPortAspectRatio
  (params (UnitRadius :type Float%20%28single-precision%29))
  (bind _aspectratio (CallFunction|GetViewportAspectRatio))
  (return (Math|Vector2D|MakeVector2D (* (Math|Float|Clamp(Float) _aspectratio 1.0 1.33) UnitRadius) (* (Math|Float|Clamp(Float) (/ 1.0 _aspectratio) 1.0 1.33) UnitRadius))))

(fn FaceFacingInput
  (bind _facingvector (CallFunction|GetFacingVector))
  (Transformation|SetActorRotation (Math|Rotator|FindLookatRotation (Math|Vector|MakeVector 0.0 0.0 0.0) _facingvector))
  (CallFunction|MatchSpringArmLocationtoFacingVector (Math|Conversions|ToVector2D(Vector) _facingvector)))