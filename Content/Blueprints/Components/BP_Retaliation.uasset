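; BP_Retaliation is a component that tracks aggressors and signals its owner to retaliate against the current one at a fixed frequency.
; The first aggressor becomes the target, and removing it promotes the next in the list, broadcasting OnAggressorChanged.
; A looping timer fires OnRetaliate, immediately on first start.
; When the list empties, the timer clears on its next tick, so a returning aggressor cannot reset the cadence.
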(fn AddAggressor
  (params (Aggressor :type Actor%20Object%20Reference))
  (if (Utilities|Time|IsTimerActivebyHandle (Variables|Default|GetRetaliationTimer))
    (Variables|Default|SetPendingRetaliationTimerClear false)
    (else
      (bind _returnvalue (Utilities|Time|SetTimerbyFunctionName 0 "TryRetaliate" (Variables|Default|GetFrequency) true))
      (Variables|Default|SetRetaliationTimer _returnvalue)
      (CallFunction|TryRetaliate)))
  (bind _returnvalue_2 (Utilities|Array|Add (Variables|Default|GetAggressors) Aggressor))
  (Utilities|When (== _returnvalue_2 0))
  (bind _output_get (Variables|Default|SetCurrentAggressor Aggressor))
  (Default|CallOnAggressorChanged _output_get))

(fn RemoveAggressor
  (params (Aggressor :type Actor%20Object%20Reference))
  (Utilities|Array|RemoveItem (Variables|Default|GetAggressors) Aggressor)
  (Utilities|When (== Aggressor (Variables|Default|GetCurrentAggressor)))
  (if (== (Utilities|Array|Length (Variables|Default|GetAggressors)) 0)
    (Variables|Default|SetCurrentAggressor 0)
    (Variables|Default|SetPendingRetaliationTimerClear true)
    (else
      (bind _output_get (Variables|Default|SetCurrentAggressor (Utilities|Array|Get(acopy) (Variables|Default|GetAggressors))))
      (Default|CallOnAggressorChanged _output_get))))

(fn TryRetaliate
  (if (Variables|Default|GetPendingRetaliationTimerClear)
    (Utilities|Time|ClearandInvalidateTimerbyHandle (Variables|Default|GetRetaliationTimer))
    (Variables|Default|SetPendingRetaliationTimerClear false)
    (else
      (Default|CallOnRetaliate (Variables|Default|GetCurrentAggressor)))))