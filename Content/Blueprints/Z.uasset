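; Game mode Z runs a timed round with Barbarians around players, reloading the level when time expires or no player has a pawn.
; Each tick updates the screen-space countdown and gathers every player's staggered-grid cell plus neighbors.
; Set difference against last tick's cells finds fresh ones, spawning one randomly offset Barbarian where none overlaps.
; Barbarians outside visible cells are destroyed, and optional debug drawing shows player 0's cells.
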(event Custom|Event%20CompleteGame
  (bind _returnvalue (Game|GetCurrentLevelName true))
  (Game|OpenLevel(byName) (Utilities|String|StringToName _returnvalue)))

(event EventInitializeHUDforPlayer
  (params (NewPlayer :type Player%20Controller%20Object%20Reference))
  (bind _returnvalue (Game|SpawnActorfromClass "/Game/Blueprints/ScreenSpaceText.ScreenSpaceText_C" (CallFunction|UnitTransform) "Undefined" 0 9.0 "(X=0.010000,Y=0.990000)" NewPlayer 0))
  (bind _output_get (Variables|Default|SetTimeRemainingDisplay _returnvalue))
  (Class|TextRenderComponent|SetVerticalAlignment (Variables|/Game/Blueprints/ScreenSpaceText.ScreenSpaceText_C|GetTextRender _output_get) "EVRTA_TextBottom")
  (CallFunction|UpdateTimeRemainingDisplay))

(event EventTick
  (params (DeltaSeconds :type Float%20%28single-precision%29))
  (bind _anyplayerpossessespawn (CallFunction|AnyPlayerPossessesPawn))
  (if _anyplayerpossessespawn
    (bind _returnvalue (CallFunction|UpdateTimeRemaining))
    (if (> _returnvalue 0.0)
      (CallFunction|UpdateTimeRemainingDisplay)
      (bind _return (CallFunction|GetVisibleCells))
      (bind _output_get (Variables|Default|SetVisibleCells _return))
      (SpawnBarbarian|SpawnBarbariansinFreshCells _output_get (Variables|Default|GetPreviousVisibleCells))
      (SpawnBarbarian|CullBarbariansinStaleCells (Variables|Default|GetVisibleCells))
      (Variables|Default|SetPreviousVisibleCells (Variables|Default|GetVisibleCells))
      (Utilities|When (Variables|Default|GetDrawDebugGeometry))
      (Debug|DrawPlayerDebugGeometry)
      (else
        (CallFunction|EventCompleteGame)))
    (else
      (CallFunction|EventCompleteGame))))

(fn ConstructionScript)

(fn SpawnCellIndexatPlayerLocation
  (params (PlayerIndex :type Integer))
  (return (SpawnCell|SpawnCellIndexatActorLocation (Game|Player|GetPlayerPawn PlayerIndex))))

(fn SpawnBarbarianTurretinSpawnCellatIndex
  (params (Index :type Int%20Point%20Structure))
  (Game|SpawnActorfromClass "/Game/Blueprints/Barbarian.Barbarian_C" (Math|Transform|MakeTransform (Math|Conversions|ToVector(Vector2D) (+ (Class|ZJoyBlueprintFunctionLibrary|StaggeredCellCenteratIndex Index (Variables|Default|GetSpawnCellSize)) (* (CallFunction|RandomUnitVector2D) (Math|Random|RandomFloatinRange 0.0 (* (SpawnCell|SpawnCellCircleRadius) 0.8)))))) "Undefined" 0 0))

(fn SpawnCellatIndexOverlapsActors
  (params (Index :type Int%20Point%20Structure))
  (bind _returnvalue (Collision|SphereOverlapActors (Math|Conversions|ToVector(Vector2D) (Class|ZJoyBlueprintFunctionLibrary|StaggeredCellCenteratIndex Index (Variables|Default|GetSpawnCellSize))) (SpawnCell|SpawnCellCircleRadius) (Utilities|Array|MakeArray "ObjectTypeQuery6" "ObjectTypeQuery2") "/Game/Blueprints/Barbarian.Barbarian_C"))
  (return _returnvalue))

(fn DrawSpawnCellatIndex
  (params (Line%20Color :type Linear%20Color%20Structure) (Index :type Int%20Point%20Structure) (Z :type Float%20%28single-precision%29))
  (CallFunction|DrawBox2D (Class|ZJoyBlueprintFunctionLibrary|StaggeredCellBoundsatIndex Index (Variables|Default|GetSpawnCellSize)) Line%20Color Z)
  (Debug|DrawSpawnCellCircle Index (Variables|Default|GetSpawnCellSize) (- Z 0.001) Line%20Color))

(fn DrawPlayerDebugGeometry
  (params (PlayerIndex :type Integer))
  (bind _returnvalue (SpawnCell|SpawnCellIndexatPlayerLocation PlayerIndex))
  (Debug|DrawSpawnCellatIndex (Variables|Default|GetPrimaryDebugColor) _returnvalue 0.001)
  (bind _result (Utilities|Set|ToArray (Class|ZJoyBlueprintFunctionLibrary|StaggeredCellNeighborsatIndex _returnvalue)))
  (for _array_element _result
    (Debug|DrawSpawnCellatIndex (Variables|Default|GetSecondaryDebugColor) _array_element 0.0)))

(fn DrawSpawnCellCircle
  (params (Index :type Int%20Point%20Structure) (CellSize :type Float%20%28single-precision%29) (Z :type Float%20%28single-precision%29) (LineColor :type Linear%20Color%20Structure))
  (Rendering|Debug|DrawDebugCircle (Math|Conversions|ToVector(Vector2D) (Class|ZJoyBlueprintFunctionLibrary|StaggeredCellCenteratIndex Index CellSize) Z) (SpawnCell|SpawnCellCircleRadius) 72 LineColor 0.0 5.0 "1.000000,0.000000,0.000000" "0.000000,1.000000,0.000000"))

(fn SpawnCellCircleRadius
  (return (* (Variables|Default|GetSpawnCellSize) 0.866)))

(fn SpawnBarbariansinCellatIndex
  (params (Index :type Int%20Point%20Structure%20%28by%20ref%29))
  (bind _returnvalue (SpawnCell|SpawnCellatIndexOverlapsActors Index))
  (Utilities|Unless _returnvalue)
  (SpawnBarbarian|SpawnBarbarianTurretinSpawnCellatIndex Index))

(fn SpawnCellIndexatActorLocation
  (params (Actor :type Actor%20Object%20Reference))
  (return (Class|ZJoyBlueprintFunctionLibrary|StaggeredCellIndexatPoint (Math|Conversions|ToVector2D(Vector) (Transformation|GetActorLocation Actor)) (Variables|Default|GetSpawnCellSize))))

(fn AnyPlayerPossessesPawn
  (bind _index (Utilities|ForEachPlayer)
    (:LoopBody
      (LocalVariables|SetAny (or (LocalVariables|GetAny) (Utilities|IsValid (Game|Player|GetPlayerPawn _index)))))
    (:Completed
      (return (LocalVariables|GetAny)))))

(fn CullBarbariansinStaleCells
  (params (VisibleCells :type Set%20of%20Int%20Point%20Structures))
  (bind _outactors (Actor|GetAllActorsOfClass "/Game/Blueprints/Barbarian.Barbarian_C"))
  (for _array_element _outactors
    (Utilities|Unless (Utilities|Set|Contains VisibleCells (SpawnCell|SpawnCellIndexatActorLocation _array_element)))
    (Actor|DestroyActor _array_element)))

(fn GetVisibleCells
  (bind _index (Utilities|ForEachPlayer)
    (:LoopBody
      (bind _result (Utilities|Set|Union (LocalVariables|GetCells) (Class|ZJoyBlueprintFunctionLibrary|StaggeredCellNeighborsatIndex (SpawnCell|SpawnCellIndexatPlayerLocation _index))))
      (bind _output_get (LocalVariables|SetCells _result))
      (Utilities|Set|Add _output_get (SpawnCell|SpawnCellIndexatPlayerLocation _index)))
    (:Completed
      (return (LocalVariables|GetCells)))))

(fn SpawnBarbariansinFreshCells
  (params (A :type Set%20of%20Int%20Point%20Structures) (B :type Set%20of%20Int%20Point%20Structures))
  (bind _result (Utilities|Set|Difference A B))
  (bind _result_2 (Utilities|Set|ToArray _result))
  (for _array_element _result_2
    (SpawnBarbarian|SpawnBarbariansinCellatIndex _array_element)))

(fn UpdateTimeRemainingDisplay
  (bind _timeremaininginseconds (Variables|Default|GetTimeRemainingInSeconds))
  (bind _returnvalue (Math|Float|Round _timeremaininginseconds))
  (Default|SetText (Variables|Default|GetTimeRemainingDisplay) (Utilities|Text|FormatText "{Minutes}:{Seconds}" (/ _returnvalue 60) (Utilities|Text|ToText(Integer) (Math|Integer|%(Integer) _returnvalue 60) false true 2))))

(fn UpdateTimeRemaining
  (bind _output_get (Variables|Default|SetTimeRemainingInSeconds (- (Variables|Default|GetTimeRemainingInSeconds) (Utilities|Time|GetWorldDeltaSeconds))))
  (return _output_get))