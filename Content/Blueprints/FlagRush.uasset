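; FlagRush spawns Barbarian turrets around players as they move, using a staggered 2D grid of spawn cells.
; Each tick, every player's current cell restarts its cooldown and neighboring cells are checked for spawning.
; A neighbor holding a Barbarian restarts its cooldown; an empty one with expired cooldown spawns one at a random offset from its center.
; A map stores cooldown expiry per cell, and optional debug drawing shows cells and cooldowns.
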(event EventBeginPlay)

(event EventTick
  (params (DeltaSeconds :type Float%20%28single-precision%29))
  (bind _index (Utilities|ForEachPlayer)
    (:LoopBody
      (SpawnBarbarian|SpawnBarbariansNearPlayer _index)
      (if (Variables|Default|GetDrawDebugGeometry)
        (Debug|DrawPlayerDebugGeometry _index)))))

(fn ConstructionScript)

(fn SpawnCellIndexatPlayerLocation
  (params (PlayerIndex :type Integer))
  (return (Class|ZJoyBlueprintFunctionLibrary|StaggeredCellIndexatPoint (Math|Conversions|ToVector2D(Vector) (Transformation|GetActorLocation (Game|Player|GetPlayerPawn PlayerIndex))) (Variables|Default|GetSpawnCellSize))))

(fn SpawnBarbarianTurretinSpawnCellatIndex
  (params (Index :type Int%20Point%20Structure))
  (Game|SpawnActorfromClass "/Game/Blueprints/Barbarian.Barbarian_C" (Math|Transform|MakeTransform (Math|Conversions|ToVector(Vector2D) (+ (Class|ZJoyBlueprintFunctionLibrary|StaggeredCellCenteratIndex Index (Variables|Default|GetSpawnCellSize)) (* (CallFunction|RandomUnitVector2D) (Math|Random|RandomFloatinRange 0.0 (* (SpawnCell|GetSpawnCellCircleRadius) 0.8))))) "0.000000,0.000000,0.000000" "1.000000,1.000000,1.000000") "Undefined" 0 0))

(fn SpawnCellatIndexReady
  (params (Index :type Int%20Point%20Structure%20%28by%20ref%29))
  (return (< (SpawnCell|SecondsTillSpawnCellatIndexActive Index) 0.0)))

(fn SpawnCellatIndexOverlapsActors
  (params (Index :type Int%20Point%20Structure))
  (bind _returnvalue (Collision|SphereOverlapActors (Math|Conversions|ToVector(Vector2D) (Class|ZJoyBlueprintFunctionLibrary|StaggeredCellCenteratIndex Index (Variables|Default|GetSpawnCellSize))) (SpawnCell|GetSpawnCellCircleRadius) (Utilities|Array|MakeArray "ObjectTypeQuery2") "/Game/Blueprints/Barbarian.Barbarian_C"))
  (return _returnvalue))

(fn SpawnBarbariansNearPlayer
  (params (PlayerIndex :type Integer))
  (bind _returnvalue (SpawnCell|SpawnCellIndexatPlayerLocation PlayerIndex))
  (SpawnCell|ResetSpawnCellCooldownatIndex _returnvalue)
  (bind _result (Utilities|Set|ToArray (Class|ZJoyBlueprintFunctionLibrary|StaggeredCellNeighborsatIndex _returnvalue)))
  (for _array_element _result
    (SpawnBarbarian|SpawnBarbariansinCellatIndex _array_element)))

(fn DrawSpawnCellatIndex
  (params (Line%20Color :type Linear%20Color%20Structure) (Index :type Int%20Point%20Structure) (Z :type Float%20%28single-precision%29))
  (CallFunction|DrawBox2D (Class|ZJoyBlueprintFunctionLibrary|StaggeredCellBoundsatIndex Index (Variables|Default|GetSpawnCellSize)) Line%20Color Z)
  (Debug|DrawSpawnCellCircle Index (Variables|Default|GetSpawnCellSize) (- Z 0.001) Line%20Color))

(fn DrawPlayerDebugGeometry
  (params (PlayerIndex :type Integer))
  (bind _returnvalue (SpawnCell|SpawnCellIndexatPlayerLocation PlayerIndex))
  (Debug|DrawSpawnCellatIndex (Variables|Default|GetPrimaryDebugColor) _returnvalue 0.001)
  (bind _result (Utilities|Set|ToArray (Class|ZJoyBlueprintFunctionLibrary|StaggeredCellNeighborsatIndex _returnvalue)))
  (for _array_element _result
    (Debug|DrawSpawnCellatIndex (Variables|Default|GetSecondaryDebugColor) _array_element 0.0)))

(fn SecondsTillSpawnCellatIndexActive
  (params (Index :type Int%20Point%20Structure%20%28by%20ref%29))
  (return (- (.Value (Utilities|Map|Find (Variables|Default|GetSpawnCellIndexToCooldownExpiry) Index)) (Utilities|Time|GetTimeSeconds))))

(fn DrawSpawnCellCircle
  (params (Index :type Int%20Point%20Structure) (CellSize :type Float%20%28single-precision%29) (Z :type Float%20%28single-precision%29) (LineColor :type Linear%20Color%20Structure))
  (Rendering|Debug|DrawDebugCircle (Math|Conversions|ToVector(Vector2D) (Class|ZJoyBlueprintFunctionLibrary|StaggeredCellCenteratIndex Index CellSize) Z) (SpawnCell|GetSpawnCellCircleRadius) 72 (* LineColor (Math|Float|MapRangeClamped (SpawnCell|SecondsTillSpawnCellatIndexActive Index) 0.0 (Variables|Default|GetSpawnCooldownSeconds) 1.0 0.0)) 0.0 5.0 "1.000000,0.000000,0.000000" "0.000000,1.000000,0.000000"))

(fn GetSpawnCellCircleRadius
  (return (* (Variables|Default|GetSpawnCellSize) 0.866)))

(fn ResetSpawnCellCooldownatIndex
  (params (Index :type Int%20Point%20Structure%20%28by%20ref%29))
  (Utilities|Map|Add (Variables|Default|GetSpawnCellIndexToCooldownExpiry) Index (+ (Variables|Default|GetSpawnCooldownSeconds) (Utilities|Time|GetTimeSeconds))))

(fn SpawnBarbariansinCellatIndex
  (params (Index :type Int%20Point%20Structure%20%28by%20ref%29))
  (bind _returnvalue (SpawnCell|SpawnCellatIndexOverlapsActors Index))
  (if _returnvalue
    (SpawnCell|ResetSpawnCellCooldownatIndex Index)
    (elif (SpawnCell|SpawnCellatIndexReady Index)
      (SpawnBarbarian|SpawnBarbarianTurretinSpawnCellatIndex Index))))