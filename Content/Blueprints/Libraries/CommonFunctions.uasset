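; Blueprint function library of small shared helpers for debug drawing, 2D math and common queries.
; Debug helpers draw an actor-space vector as a red line and 2D boxes as four edges through DrawDebugLine2D, which lifts 2D points to a given Z.
; Other functions return the viewport aspect ratio, a random unit 2D vector from a rotated X axis, an identity transform and a target's current frame number.
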(fn DrawDebugVectorinActorSpace
  (params (Vector :type Vector) (Actor :type Actor%20Object%20Reference))
  (bind _returnvalue (Transformation|GetActorLocation Actor))
  (Rendering|Debug|DrawDebugLine 0 _returnvalue (+ _returnvalue (Math|Vector|RotateVector Vector (Transformation|GetActorRotation Actor))) "(R=1.000000,G=0.000000,B=0.000000,A=1.000000)" 0.0))

(fn GetViewportAspectRatio
  (bind ___worldcontext (LocalVariables|Get__WorldContext))
  (bind _returnvalue (Viewport|GetViewportSize ___worldcontext))
  (bind (_x _y) (Math|Vector2D|BreakVector2D _returnvalue))
  (return (/ _x _y)))

(fn DrawBox2D
  (params (Box2D :type Box%202D%20Structure%20%28by%20ref%29) (LineColor :type Linear%20Color%20Structure) (Z :type Float%20%28single-precision%29))
  (bind (_min _max) (Utilities|Struct|BreakBox2D Box2D))
  (bind ___worldcontext (LocalVariables|Get__WorldContext))
  (bind (_x _y) (Math|Vector2D|BreakVector2D _max))
  (bind (_x_2 _y_2) (Math|Vector2D|BreakVector2D _min))
  (bind _returnvalue (Math|Vector2D|MakeVector2D _x _y))
  (bind _returnvalue_2 (Math|Vector2D|MakeVector2D _x_2 _y_2))
  (bind _returnvalue_3 (Math|Vector2D|MakeVector2D _x_2 _y))
  (bind _returnvalue_4 (Math|Vector2D|MakeVector2D _x _y_2))
  (Debug|DrawDebugLine2D _returnvalue_2 _returnvalue_3 Z LineColor ___worldcontext)
  (Debug|DrawDebugLine2D _returnvalue_3 _returnvalue Z LineColor ___worldcontext)
  (Debug|DrawDebugLine2D _returnvalue _returnvalue_4 Z LineColor ___worldcontext)
  (Debug|DrawDebugLine2D _returnvalue_4 _returnvalue_2 Z LineColor ___worldcontext))

(fn DrawDebugLine2D
  (params (LineStart :type Vector%202D%20Structure) (LineEnd :type Vector%202D%20Structure) (Z :type Float%20%28single-precision%29) (LineColor :type Linear%20Color%20Structure))
  (Rendering|Debug|DrawDebugLine 0 (Math|Conversions|ToVector(Vector2D) LineStart Z) (Math|Conversions|ToVector(Vector2D) LineEnd Z) LineColor 0.0 5.0))

(fn RandomUnitVector2D
  (return (Class|KismetMathLibrary|GetRotated2D (Math|Vector2D|MakeVector2D 1.0 0.0) (Math|Random|RandomFloatinRange 0.0 3.6e+02))))

(fn UnitTransform
  (return (Math|Transform|MakeTransform "0, 0, 0")))

(fn GetCurrentFrame
  (params (Target :type Movie%20Scene%20Sequence%20Player%20Object%20Reference))
  (return (.value (.frame (Sequencer|Player|GetCurrentTime Target)))))