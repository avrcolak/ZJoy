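; BP_GuardLine is a controller that makes its pawn guard a line around the controller's own location.
; GuardBox overlaps add and remove aggressors on the Retaliation component, which drives facing and triggers the pawn's ShootMessage.
; Each tick the pawn moves toward the aggressor's position projected onto the guard's axes, matching it sideways but only halfway forward, or returns to origin when none remains.
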(event OnComponentBeginOverlap(GuardBox)
  (params (OverlappedComponent :type Primitive%20Component%20Object%20Reference) (OtherActor :type Actor%20Object%20Reference) (OtherComp :type Primitive%20Component%20Object%20Reference) (OtherBodyIndex :type Integer) (bFromSweep :type Boolean) (SweepResult :type Hit%20Result%20Structure%20%28by%20ref%29))
  (Default|AddAggressor (Variables|Default|GetRetaliation) OtherActor))

(event OnComponentEndOverlap(GuardBox)
  (params (OverlappedComponent :type Primitive%20Component%20Object%20Reference) (OtherActor :type Actor%20Object%20Reference) (OtherComp :type Primitive%20Component%20Object%20Reference) (OtherBodyIndex :type Integer))
  (Default|RemoveAggressor (Variables|Default|GetRetaliation) OtherActor))

(event OnRetaliate(Retaliation)
  (params (Aggressor :type Actor%20Object%20Reference))
  (Class|BPIShoots|Shoot(Message) (Pawn|GetControlledPawn) "0, 0, 0"))

(event OnAggressorChanged(Retaliation)
  (params (Aggressor :type Actor%20Object%20Reference))
  (Pawn|SetControlRotation (Math|Rotator|FindLookatRotation (Transformation|GetActorLocation) (Transformation|GetActorLocation Aggressor))))

(event EventTick
  (params (DeltaSeconds :type Float%20%28single-precision%29))
  (Utilities|IsValid (Pawn|GetControlledPawn)
    (:Is%20Valid
      (Utilities|IsValid (Variables|/Game/Blueprints/Components/BP_Retaliation.BP_Retaliation_C|GetCurrentAggressor (Variables|Default|GetRetaliation))
        (:Is%20Valid
          (CallFunction|MovePawntoAggressor))
        (:Is%20Not%20Valid
          (CallFunction|MovePawntoOrigin))))))

(event EventPossess
  (params (PossessedPawn :type Pawn%20Object%20Reference))
  (Default|RemoveAggressor (Variables|Default|GetRetaliation) PossessedPawn))

(fn ConstructionScript)

(fn MovePawntoAggressor
  (bind _returnvalue (Transformation|GetActorLocation))
  (bind _returnvalue_2 (Pawn|GetControlledPawn))
  (bind _retaliation (Variables|Default|GetRetaliation))
  (bind _currentaggressor (Variables|/Game/Blueprints/Components/BP_Retaliation.BP_Retaliation_C|GetCurrentAggressor _retaliation))
  (bind _returnvalue_3 (Transformation|GetActorLocation _currentaggressor))
  (bind _returnvalue_4 (- _returnvalue_3 _returnvalue))
  (Pawn|Input|AddMovementInput _returnvalue_2 (/ (- (+ (Math|Vector|ProjectVectorontoVector _returnvalue_4 (Transformation|GetActorRightVector)) (* (Math|Vector|ProjectVectorontoVector _returnvalue_4 (Transformation|GetActorForwardVector)) 0.5) (Transformation|GetActorLocation)) (Transformation|GetActorLocation _returnvalue_2)) 5e+01) 1.0 true))

(fn MovePawntoOrigin
  (bind _returnvalue (Pawn|GetControlledPawn))
  (Pawn|Input|AddMovementInput _returnvalue (/ (- (Transformation|GetActorLocation) (Transformation|GetActorLocation _returnvalue)) 5e+01) 1.0 false))