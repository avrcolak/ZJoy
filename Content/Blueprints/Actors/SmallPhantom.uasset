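; SmallPhantom is a small phantom pawn that flies by its own movement code and fires bullets while alive.
; Each tick, Move consumes pending movement input and interpolates location and rotation at constant speeds toward the input offset and control rotation.
; Tick then derives CurrentVelocity from the frame's position change, a per-frame delta not divided by time, exposed through Velocity.
; The Shoot event spawns a bullet.
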(event EventShoot
  (params (Target :type Vector :default "0, 0, 0"))
  (Utilities|When (Variables|Default|GetAlive))
  (CallFunction|SpawnBullet 1.6e+03))

(event EventTick
  (params (DeltaSeconds :type Float%20%28single-precision%29))
  (|CallParentFunction DeltaSeconds)
  (Utilities|When (Variables|Default|GetAlive))
  (Utilities|FlowControl|Sequence
    (:then_0
      (CallFunction|Move))
    (:then_1
      (Variables|Default|SetCurrentVelocity (- (Transformation|GetActorLocation) (Variables|Default|GetPreviousLocation)))
      (Variables|Default|SetPreviousLocation (Transformation|GetActorLocation)))))

(fn ConstructionScript)

(fn Move
  (bind _returnvalue (Transformation|GetActorLocation))
  (bind _returnvalue_2 (Class|Pawn|ConsumeMovementInputVector))
  (Transformation|SetActorLocationAndRotation (Math|Interpolation|VInterptoConstant _returnvalue (+ _returnvalue_2 _returnvalue) (Utilities|Time|GetWorldDeltaSeconds) (Variables|Default|GetSpeed)) (Class|KismetMathLibrary|RInterptoConstant (Transformation|GetActorRotation) (Pawn|GetControlRotation :!class /Script/Engine.Pawn) (Utilities|Time|GetWorldDeltaSeconds) (Variables|Default|GetRotationSpeed))))

(fn Velocity
  (return (Variables|Default|GetCurrentVelocity)))