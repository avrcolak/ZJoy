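; Player controller for the human player, steering and firing the hero ship and showing score and lives as spawned screen-space actors.
; Each tick it turns mouse or stick input, switching automatically between them, into a camera-relative control rotation and feeds the magnitude to the ship.
; It also handles camera roll, speed cycling and quit.
; Possession builds life icons that death events remove; unpossession clears them and possesses a placeholder pawn at the old camera.
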(event Custom|RemoveHudLife
  (bind _hudlives (Variables|Default|GetHudLives))
  (Utilities|Unless (Utilities|IsEmpty (Variables|Default|GetHudLives)))
  (Actor|DestroyActor (Utilities|GetLast _hudlives))
  (Utilities|RemoveLast _hudlives))

(event EventBeginPlay
  (bind _returnvalue (Game|SpawnActorfromClass "/Game/Blueprints/Actors/BP_ScreenSpaceText.BP_ScreenSpaceText_C" (CallFunction|UnitTransform) "Undefined" 0 9.0 "(X=0.990000,Y=0.010000)" self 0))
  (bind _output_get (Variables|Default|SetScoreDisplay _returnvalue))
  (Rendering|Components|TextRender|SetHorizontalAlignment (Variables|/Game/Blueprints/Actors/BP_ScreenSpaceText.BP_ScreenSpaceText_C|GetTextRender _output_get) "EHTA_Right")
  (CallFunction|UpdateScoreDisplay))

(event EventTick
  (params (DeltaSeconds :type Float%20%28single-precision%29))
  (bind (_direction _magnitude) (CallFunction|FacingVector))
  (bind (_x _y) (Math|Vector2D|BreakVector2D _direction))
  (Class|ZJoyBlueprintFunctionLibrary|MaintainMinorAxisFov self)
  (CallFunction|UpdateMousePosition)
  (Utilities|WhenControlsPawn)
  (CallFunction|RotatePawn _x _y)
  (bind _ashero_ship (Utilities|WhenControlledPawnIsHeroShip))
  (Variables|/Game/Blueprints/Actors/BP_HeroShip.BP_HeroShip_C|SetFacingInputMagnitude _ashero_ship _magnitude))

(event EventUnPossess
  (params (UnpossessedPawn :type Pawn%20Object%20Reference))
  (Utilities|IsValid UnpossessedPawn
    (:Is%20Valid
      (CallFunction|DestroyHudLives)
      (bind _returnvalue (Game|SpawnActorfromClass "/Script/Engine.Pawn" (Transformation|GetWorldTransform (Actor|GetComponentbyClass UnpossessedPawn "/Script/Engine.CameraComponent")) "Undefined" 0 0))
      (Pawn|Possess _returnvalue))))

(event EventAddScore
  (params (Score :type Integer))
  (CallFunction|IncrementScore Score))

(event EventPossess
  (params (PossessedPawn :type Pawn%20Object%20Reference))
  (bind _validobject (Utilities|WhenValid PossessedPawn))
  (bind _validobject_2 (Utilities|WhenValid (Actor|GetComponentbyClass _validobject "/Game/Blueprints/Components/BP_Death.BP_Death_C")))
  (EventDispatchers|BindEventtoOnDeath _validobject_2 (delegate Custom|RemoveHudLife))
  (bind _numberoflives (Class|BPIDies|NumberOfLives(Message) _validobject))
  (CallFunction|SpawnHudLives _numberoflives))

(event Input|ActionEvents|InputActionShoot
  (params (Key :type Key%20Structure))
  (:Pressed
    (bind _ashero_ship (Utilities|WhenControlledPawnIsHeroShip))
    (Default|StartShooting _ashero_ship))
  (:Released
    (bind _ashero_ship_2 (Utilities|WhenControlledPawnIsHeroShip))
    (Default|StopShooting _ashero_ship_2)))

(event Input|ActionEvents|InputActionCycleSpeed
  (params (Key :type Key%20Structure))
  (:Pressed
    (Utilities|WhenControlsPawn)
    (Class|BPICyclesSpeeds|CycleSpeedMultiplier(Message) (Pawn|GetControlledPawn))))

(event Input|AxisEvents|InputAxisFaceUp
  (params (AxisValue :type Float%20%28single-precision%29))
  (Utilities|WhenControlsPawn)
  (bind _output_get (Variables|Default|SetFaceUp AxisValue))
  (Utilities|Unless (Math|Float|NearlyEqual(Float) _output_get 0.0 1e-06))
  (CallFunction|StopUsingMouse))

(event Input|AxisEvents|InputAxisFaceRight
  (params (AxisValue :type Float%20%28single-precision%29))
  (Utilities|WhenControlsPawn)
  (bind _output_get (Variables|Default|SetFaceRight AxisValue))
  (Utilities|Unless (Math|Float|NearlyEqual(Float) _output_get 0.0 1e-06))
  (CallFunction|StopUsingMouse))

(event Input|AxisEvents|InputAxisRotateCameraRight
  (params (AxisValue :type Float%20%28single-precision%29))
  (bind _returnvalue (Pawn|GetControlledPawn))
  (bind _returnvalue_2 (Actor|GetComponentbyClass _returnvalue "/Script/Engine.CameraComponent"))
  (Utilities|WhenControlsPawn)
  (Utilities|IsValid _returnvalue_2
    (:Is%20Valid
      (Transformation|AddLocalRotation _returnvalue_2 (Math|Rotator|MakeRotator (* (Utilities|Time|GetWorldDeltaSeconds) (* AxisValue (Variables|Default|GetRotationSpeed))) 0.0 0.0) false false))))

(event Input|KeyboardEvents|Escape
  (params (Key :type Key%20Structure))
  (:Pressed
    (Game|QuitGame self "Quit" false)))

(event Input|MouseEvents|LeftMouseButton
  (params (Key :type Key%20Structure))
  ;[1 1 1] Hack to prevent losing focus on click
  (:Released
    (Input|SetInputModeGameandUI self 0 "LockAlways" false)))

(fn ConstructionScript)

(fn IncrementScore
  (params (Amount :type Integer))
  (Variables|Default|SetScore (+ Amount (Variables|Default|GetScore)))
  (CallFunction|UpdateScoreDisplay))

(fn RotatePawn
  (params (Right :type Float%20%28single-precision%29) (Up :type Float%20%28single-precision%29))
  (bind _playercameramanager (Variables|Default|GetPlayerCameraManager))
  (bind _returnvalue (Camera|GetCameraRotation _playercameramanager))
  (Utilities|Unless (Class|KismetMathLibrary|IsNearlyZero2D (Math|Vector2D|MakeVector2D Right Up) 0.0001))
  (Pawn|SetControlRotation (Math|Rotator|FindLookatRotation (Math|Vector|MakeVector 0.0 0.0 0.0) (+ (* (Math|Vector|GetUpVector _returnvalue) Up) (* (Math|Vector|GetRightVector _returnvalue) Right)))))

(fn GetNormalizedMousePositionfromViewportCenter
  (bind (_locationx _locationy _returnvalue) (Game|Player|GetMousePosition))
  (bind _returnvalue_2 (Viewport|GetViewportSize))
  (bind _returnvalue_3 (* _returnvalue_2 0.5))
  (bind _returnvalue_4 (Math|Vector2D|MakeVector2D _locationx _locationy))
  (bind _y (Math|Vector2D|BreakVector2D _returnvalue_2))
  (bind _returnvalue_5 (- _returnvalue_4 _returnvalue_3))
  (bind _returnvalue_6 (/ _returnvalue_5 _y))
  (bind _returnvalue_7 (* _returnvalue_6 2.0))
  (return _returnvalue (Math|Vector2D|MakeVector2D (.x _returnvalue_7) (.y _returnvalue_7))))

(fn StopUsingMouse
  (Variables|Default|SetPlayerUsingMouse false)
  (Variables|Default|SetbShowMouseCursor false)
  (Input|SetInputModeGameandUI self 0 "LockAlways" false) ; Hack to ensure mouse cursor gets hidden
)

(fn StartUsingMouse
  (Variables|Default|SetPlayerUsingMouse true)
  (Variables|Default|SetbShowMouseCursor true))

(fn UpdateScoreDisplay
  (Default|SetText (Variables|Default|GetScoreDisplay) (Utilities|Text|ToText(Integer) (Variables|Default|GetScore))))

(fn FacingVector
  (bind _returnvalue (Class|KismetMathLibrary|Vector2DZero))
  (bind _mouseposition (Variables|Default|GetMousePosition))
  (bind _faceright (Variables|Default|GetFaceRight))
  (bind _faceup (Variables|Default|GetFaceUp))
  (bind _playerusingmouse (Variables|Default|GetPlayerUsingMouse))
  (bind _returnvalue_2 (Math|Vector2D|MakeVector2D _faceright _faceup))
  (bind _returnvalue_3 (* (.y _mouseposition) -1.0))
  (bind _returnvalue_4 (Class|KismetMathLibrary|VSize2DSquared _returnvalue_2))
  (bind _returnvalue_5 (Math|Vector2D|MakeVector2D (.x _mouseposition) _returnvalue_3))
  (bind _returnvalue_6 (< _returnvalue_4 0.025))
  (bind _returnvalue_7 (select _returnvalue_6 _returnvalue _returnvalue_2))
  (bind _returnvalue_8 (select _playerusingmouse _returnvalue_5 _returnvalue_7))
  (return (Math|Vector2D|Normalize2D _returnvalue_8) (Math|Vector2D|Vector2DLength _returnvalue_8)))

(fn UpdateMousePosition
  (bind (_returnvalue _mouseposition) (CallFunction|GetNormalizedMousePositionfromViewportCenter))
  (Utilities|When _returnvalue)
  (bind _output_get (Variables|Default|SetMousePosition _mouseposition))
  (if (Class|KismetMathLibrary|IsNearlyZero2D (- _output_get (Variables|Default|GetPreviousMousePosition)) 0.0001)
    _
    (else
      (CallFunction|StartUsingMouse)))
  (Variables|Default|SetPreviousMousePosition (Variables|Default|GetMousePosition)))

(fn SpawnHudLives
  (params (Lives :type Integer))
  (for _index (range 0 (- Lives 1))
    (bind _returnvalue (Game|SpawnActorfromClass "/Game/Blueprints/Actors/BP_HeroShipHudLife.BP_HeroShipHudLife_C" (CallFunction|UnitTransform) "Undefined" 0 1e+01 (Math|Vector2D|MakeVector2D (+ (* _index 0.03) 0.03) 0.03) self 0))
    (Utilities|Array|Add (Variables|Default|GetHudLives) _returnvalue)))

(fn DestroyHudLives
  (for _array_element (Variables|Default|GetHudLives)
    (Actor|DestroyActor _array_element)))