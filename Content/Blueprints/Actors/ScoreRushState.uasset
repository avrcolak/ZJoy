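; Game state for a timed Score Rush mode that gives each player a HeroShip and countdown HUD on sync, then reloads the level when time runs out.
; While heroes exist, Tick updates the timer and diffs the staggered grid cells around them against the previous frame.
; Newly visible cells without overlapping actors randomly get a guarded SmallPhantom or an Arena.
; Stale-cell cleanup is disconnected, so spawned content is never removed here.
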(event Custom|Event%20CompleteGame
  (Utilities|FlowControl|Delay 1.0)
  (bind _returnvalue (Game|GetCurrentLevelName true))
  (Game|OpenLevel(byName) (Utilities|String|StringToName _returnvalue)))

(event EventTick
  (params (DeltaSeconds :type Float%20%28single-precision%29))
  (Utilities|Unless (Networking|IsDedicatedServer))
  (bind _anyheroesexist (CallFunction|AnyHeroesExist))
  (if _anyheroesexist
    (bind _returnvalue (CallFunction|UpdateTimeRemaining))
    (if (> _returnvalue 0.0)
      (Utilities|FlowControl|Sequence
        (:then_0
          (Utilities|Unless (Networking|IsDedicatedServer))
          (CallFunction|UpdateTimeRemainingDisplay))
        (:then_1
          (bind _return (CallFunction|GetVisibleCells))
          (bind _output_get (Variables|Default|SetVisibleCells _return))
          (CellPopulation|PopulateFreshCells _output_get (Variables|Default|GetPreviousVisibleCells))
          (CellPopulation|DepopulateStaleCells (Variables|Default|GetVisibleCells))
          (Variables|Default|SetPreviousVisibleCells (Variables|Default|GetVisibleCells))
          (Utilities|When (Variables|Default|GetDrawDebugGeometry))
          (Debug|DrawNeighboringSpawnCells)))
      (else
        (CallFunction|EventCompleteGame)))))

(event EventOnSync
  (bind _outactors (Actor|GetAllActorsOfClass "/Script/ZJoy.NetPlayPlayerController"))
  (for _array_element _outactors
    (CallFunction|InitializeHUDforPlayer _array_element)
    (bind _returnvalue (Game|SpawnActorfromClass "/Game/Blueprints/Actors/HeroShip.HeroShip_C" (CallFunction|UnitTransform) "Undefined" 0 0))
    (Class|NetPlayPlayerController|PossessQuickandDirty _array_element _returnvalue)))

(fn ConstructionScript)

(fn SpawnGuardinCellatIndex
  (params (Index :type Int%20Point%20Structure))
  (bind _output_get (LocalVariables|SetSpawnTransform (CellPopulation|SpawnTransformatIndex Index)))
  (bind _returnvalue (Game|SpawnActorfromClass "/Game/Blueprints/Actors/SmallPhantom.SmallPhantom_C" _output_get "Undefined" 0 0))
  (LocalVariables|SetGuard _returnvalue)
  (bind _returnvalue_2 (Game|SpawnActorfromClass "/Game/Blueprints/Actors/GuardLine.GuardLine_C" (LocalVariables|GetSpawnTransform) "Undefined" 0 0))
  (Components|Box|SetBoxExtent (Variables|/Game/Blueprints/Actors/GuardLine.GuardLine_C|GetGuardBox _returnvalue_2) "200.000000,1000.000000,100.000000" true)
  (Class|NetPlayAIController|PossessQuickandDirty _returnvalue_2 (LocalVariables|GetGuard)))

(fn SpawnCellatIndexOverlapsActors
  (params (Index :type Int%20Point%20Structure))
  (bind _returnvalue (Collision|SphereOverlapActors (Math|Conversions|ToVector(Vector2D) (Class|ZJoyBlueprintFunctionLibrary|StaggeredCellCenteratIndex Index (Variables|Default|GetSpawnCellSize))) (SpawnCell|SpawnCellCircleRadius) (Utilities|Array|MakeArray "ObjectTypeQuery10" "ObjectTypeQuery8") 0))
  (return _returnvalue))

(fn DrawSpawnCellatIndex
  (params (Line%20Color :type Linear%20Color%20Structure) (Index :type Int%20Point%20Structure) (Z :type Float%20%28single-precision%29))
  (CallFunction|DrawBox2D (Class|ZJoyBlueprintFunctionLibrary|StaggeredCellBoundsatIndex Index (Variables|Default|GetSpawnCellSize)) Line%20Color Z)
  (Debug|DrawSpawnCellCircle Index (Variables|Default|GetSpawnCellSize) (- Z 0.001) Line%20Color))

(fn DrawNeighboringSpawnCells
  (params (Actor :type Actor%20Object%20Reference))
  (Debug|DrawSpawnCellatIndex :Line%20Color (Variables|Default|GetPrimaryDebugColor) :Z 0.001)
  (bind _result (Utilities|Set|ToArray (Class|ZJoyBlueprintFunctionLibrary|StaggeredCellNeighborsatIndex (SpawnCell|SpawnCellIndexatActorLocation Actor))))
  (for _array_element _result
    (Debug|DrawSpawnCellatIndex (Variables|Default|GetSecondaryDebugColor) _array_element 0.0)))

(fn DrawSpawnCellCircle
  (params (Index :type Int%20Point%20Structure) (CellSize :type Float%20%28single-precision%29) (Z :type Float%20%28single-precision%29) (LineColor :type Linear%20Color%20Structure))
  (Rendering|Debug|DrawDebugCircle (Math|Conversions|ToVector(Vector2D) (Class|ZJoyBlueprintFunctionLibrary|StaggeredCellCenteratIndex Index CellSize) Z) (SpawnCell|SpawnCellCircleRadius) 72 LineColor 0.0 5.0 "1.000000,0.000000,0.000000" "0.000000,1.000000,0.000000"))

(fn SpawnCellCircleRadius
  (return (* (Variables|Default|GetSpawnCellSize) 0.866)))

(fn PopulateCellatIndex
  (params (Index :type Int%20Point%20Structure%20%28by%20ref%29))
  (bind _returnvalue (SpawnCell|SpawnCellatIndexOverlapsActors Index))
  (Utilities|Unless _returnvalue)
  (Utilities|FlowControl|MultiGate true false -1
    (:Out%200
      (CellPopulation|SpawnGuardinCellatIndex Index))
    (:Out%201
      (Game|SpawnActorfromClass "/Game/Blueprints/Actors/Arena.Arena_C" (CellPopulation|SpawnTransformatIndex Index) "Undefined" 0 0))))

(fn SpawnCellIndexatActorLocation
  (params (Actor :type Actor%20Object%20Reference))
  (return (Class|ZJoyBlueprintFunctionLibrary|StaggeredCellIndexatPoint (Math|Conversions|ToVector2D(Vector) (Transformation|GetActorLocation Actor)) (Variables|Default|GetSpawnCellSize))))

(fn AnyHeroesExist
  (bind _outactors (Actor|GetAllActorsOfClass "/Game/Blueprints/Actors/HeroShip.HeroShip_C"))
  (return (not (Utilities|IsEmpty _outactors))))

(fn DepopulateStaleCells
  (params (VisibleCells :type Set%20of%20Int%20Point%20Structures)))

(fn GetVisibleCells
  (bind _outactors (Actor|GetAllActorsOfClass "/Game/Blueprints/Actors/HeroShip.HeroShip_C"))
  (for _array_element _outactors
    (bind _result (Utilities|Set|Union (LocalVariables|GetCells) (Class|ZJoyBlueprintFunctionLibrary|StaggeredCellNeighborsatIndex (SpawnCell|SpawnCellIndexatActorLocation _array_element))))
    (bind _output_get (LocalVariables|SetCells _result))
    (Utilities|Set|Add :TargetSet _output_get))
  (return (LocalVariables|GetCells)))

(fn PopulateFreshCells
  (params (A :type Set%20of%20Int%20Point%20Structures) (B :type Set%20of%20Int%20Point%20Structures))
  (bind _result (Utilities|Set|Difference A B))
  (bind _result_2 (Utilities|Set|ToArray _result))
  (for _array_element _result_2
    (CellPopulation|PopulateCellatIndex _array_element)))

(fn UpdateTimeRemainingDisplay
  (bind _timeremaininginseconds (Variables|Default|GetTimeRemainingInSeconds))
  (bind _returnvalue (Math|Float|Round _timeremaininginseconds))
  (Default|SetText (Variables|Default|GetTimeRemainingDisplay) (Utilities|Text|FormatText "{Minutes}:{Seconds}" (/ _returnvalue 60) (Utilities|Text|ToText(Integer) (Math|Integer|%(Integer) _returnvalue 60) false true 2))))

(fn UpdateTimeRemaining
  (bind _output_get (Variables|Default|SetTimeRemainingInSeconds (- (Variables|Default|GetTimeRemainingInSeconds) (Utilities|Time|GetWorldDeltaSeconds))))
  (return _output_get))

(fn SpawnTransformatIndex
  (params (Index :type Int%20Point%20Structure))
  (bind _spawncellsize (Variables|Default|GetSpawnCellSize))
  (bind _returnvalue (Class|ZJoyBlueprintFunctionLibrary|StaggeredCellCenteratIndex Index _spawncellsize))
  (return (Math|Transform|MakeTransform (Math|Vector|MakeVector (.x _returnvalue) (.y _returnvalue) 0.0))))

(fn InitializeHUDforPlayer
  (params (PlayerController :type Player%20Controller%20Object%20Reference))
  (bind _returnvalue (Game|SpawnActorfromClass "/Game/Blueprints/Actors/ScreenSpaceText.ScreenSpaceText_C" (CallFunction|UnitTransform) "Undefined" 0 9.0 "(X=0.010000,Y=0.990000)" PlayerController 0))
  (bind _output_get (Variables|Default|SetTimeRemainingDisplay _returnvalue))
  (Class|TextRenderComponent|SetVerticalAlignment (Variables|/Game/Blueprints/Actors/ScreenSpaceText.ScreenSpaceText_C|GetTextRender _output_get) "EVRTA_TextBottom")
  (CallFunction|UpdateTimeRemainingDisplay))