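; GuardLine controls a pawn that guards an area around the line's own location, shooting when its Retaliation component fires.
; Player-controlled pawns entering GuardBox register as aggressors and are removed on exit; a possessed pawn is also removed.
; Each tick, the guard interpolates toward the current aggressor's offset, projected fully on the right axis and halved on the forward axis, or drifts more slowly back to origin.
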(event OnComponentBeginOverlap(GuardBox)
  (params (OverlappedComponent :type Primitive%20Component%20Object%20Reference) (OtherActor :type Actor%20Object%20Reference) (OtherComp :type Primitive%20Component%20Object%20Reference) (OtherBodyIndex :type Integer) (bFromSweep :type Boolean) (SweepResult :type Hit%20Result%20Structure%20%28by%20ref%29))
  (bind _aspawn (Utilities|Casting|CastToPawn OtherActor))
  (Utilities|When (Pawn|IsPlayerControlled _aspawn))
  (Default|AddAggressor (Variables|Default|GetRetaliation) _aspawn))

(event OnComponentEndOverlap(GuardBox)
  (params (OverlappedComponent :type Primitive%20Component%20Object%20Reference) (OtherActor :type Actor%20Object%20Reference) (OtherComp :type Primitive%20Component%20Object%20Reference) (OtherBodyIndex :type Integer))
  (Default|RemoveAggressor (Variables|Default|GetRetaliation) OtherActor))

(event OnRetaliate(Retaliation)
  (params (Aggressor :type Actor%20Object%20Reference))
  (Class|Shoots|Shoot(Message) (Pawn|GetControlledPawn) "0, 0, 0"))

(event EventBeginPlay)

(event EventTick
  (params (DeltaSeconds :type Float%20%28single-precision%29))
  (Utilities|IsValid (Pawn|GetControlledPawn)
    (:Is%20Valid
      (Utilities|IsValid (Variables|/Game/Blueprints/Components/Retaliation.Retaliation_C|GetCurrentAggressor (Variables|Default|GetRetaliation))
        (:Is%20Valid
          (CallFunction|MovePawnTowardsAggressor))
        (:Is%20Not%20Valid
          (CallFunction|MovePawnTowardsOrigin))))))

(event EventPossess
  (params (PossessedPawn :type Pawn%20Object%20Reference))
  (Default|RemoveAggressor (Variables|Default|GetRetaliation) PossessedPawn))

(fn ConstructionScript)

(fn MovePawnTowardsAggressor
  (bind _returnvalue (Transformation|GetActorLocation))
  (bind _returnvalue_2 (Pawn|GetControlledPawn))
  (bind _retaliation (Variables|Default|GetRetaliation))
  (bind _currentaggressor (Variables|/Game/Blueprints/Components/Retaliation.Retaliation_C|GetCurrentAggressor _retaliation))
  (bind _returnvalue_3 (Transformation|GetActorLocation _currentaggressor))
  (bind _returnvalue_4 (- _returnvalue_3 _returnvalue))
  (bind _asmoves (Utilities|Casting|CastToMoves _returnvalue_2))
  (Default|Moveto _asmoves (Math|Interpolation|VInterpTo (Transformation|GetActorLocation _returnvalue_2) (+ (Math|Vector|ProjectVectorontoVector _returnvalue_4 (Transformation|GetActorRightVector)) (* (Math|Vector|ProjectVectorontoVector _returnvalue_4 (Transformation|GetActorForwardVector)) 0.5) (Transformation|GetActorLocation)) (Utilities|Time|GetWorldDeltaSeconds) 3.0)))

(fn MovePawnTowardsOrigin
  (bind _returnvalue (Pawn|GetControlledPawn))
  (Class|Moves|Moveto(Message) _returnvalue (Math|Interpolation|VInterpTo (Transformation|GetActorLocation _returnvalue) (Transformation|GetActorLocation) (Utilities|Time|GetWorldDeltaSeconds) 0.5)))