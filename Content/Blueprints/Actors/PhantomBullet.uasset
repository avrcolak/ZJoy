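; PhantomBullet is a projectile actor that destroys itself when its hit box hits something.
; The construction script passes Speed to the BulletMovement component and creates a dynamic material instance for the bullet.
; Two seconds before its initial lifespan ends, it disables hit box collision and plays a Fade timeline that drives the material's Opacity, leaving it harmless while it fades.
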(event OnComponentHit(HitBox)
  (params (HitComponent :type Primitive%20Component%20Object%20Reference) (OtherActor :type Actor%20Object%20Reference) (OtherComp :type Primitive%20Component%20Object%20Reference) (NormalImpulse :type Vector :default "0, 0, 0") (Hit :type Hit%20Result%20Structure%20%28by%20ref%29))
  (Actor|DestroyActor))

(event EventBeginPlay
  (Utilities|FlowControl|Delay (- (Variables|Actor|GetInitialLifeSpan) 2.0))
  (Collision|SetCollisionEnabled (Variables|Default|GetHitBox) "NoCollision")
  (bind _opacity (Timeline|Fade Play)
    (:Update
      (Rendering|Material|SetScalarParameterValue (Variables|Default|GetBulletMaterial) "Opacity" _opacity :!class /Script/Engine.MaterialInstanceDynamic))))

(fn ConstructionScript
  (Variables|/Game/Blueprints/Components/BulletMovement.BulletMovement_C|SetSpeed (Variables|Default|GetBulletMovement) (Variables|Default|GetSpeed))
  (bind _returnvalue (Rendering|Material|CreateDynamicMaterialInstance (Variables|Default|GetBullet) 0 0 "None" :!class /Script/Engine.PrimitiveComponent))
  (Variables|Default|SetBulletMaterial _returnvalue))