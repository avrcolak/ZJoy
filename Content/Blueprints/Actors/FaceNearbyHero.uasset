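; Controller that turns its possessed pawn's control rotation toward a nearby aggressor, or along its direction of travel when there is none.
; Each tick it snaps itself to the pawn's transform, so its Trigger volume follows the pawn.
; Trigger overlaps add and remove actors in the Retaliation component, which supplies the current aggressor; possession removes the pawn itself.
; Without an aggressor, rotation comes from the pawn's VelocityMessage and up vector.
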(event OnComponentBeginOverlap(Trigger)
  (params (OverlappedComponent :type Primitive%20Component%20Object%20Reference) (OtherActor :type Actor%20Object%20Reference) (OtherComp :type Primitive%20Component%20Object%20Reference) (OtherBodyIndex :type Integer) (bFromSweep :type Boolean) (SweepResult :type Hit%20Result%20Structure%20%28by%20ref%29))
  (Default|AddAggressor (Variables|Default|GetRetaliation) OtherActor))

(event OnComponentEndOverlap(Trigger)
  (params (OverlappedComponent :type Primitive%20Component%20Object%20Reference) (OtherActor :type Actor%20Object%20Reference) (OtherComp :type Primitive%20Component%20Object%20Reference) (OtherBodyIndex :type Integer))
  (Default|RemoveAggressor (Variables|Default|GetRetaliation) OtherActor))

(event EventBeginPlay)

(event EventTick
  (params (DeltaSeconds :type Float%20%28single-precision%29))
  (Transformation|SetActorTransform (Transformation|GetActorTransform (Pawn|GetControlledPawn)))
  (Utilities|IsValid (Pawn|GetControlledPawn)
    (:Is%20Valid
      (Utilities|IsValid (Variables|/Game/Blueprints/Components/Retaliation.Retaliation_C|GetCurrentAggressor (Variables|Default|GetRetaliation))
        (:Is%20Valid
          (CallFunction|FaceAggressor))
        (:Is%20Not%20Valid
          (CallFunction|FaceCourse))))))

(event EventPossess
  (params (PossessedPawn :type Pawn%20Object%20Reference))
  (Default|RemoveAggressor (Variables|Default|GetRetaliation) PossessedPawn))

(fn ConstructionScript)

(fn FaceAggressor
  (Pawn|SetControlRotation (Math|Rotator|FindLookatRotation (Transformation|GetActorLocation (Pawn|GetControlledPawn)) (Transformation|GetActorLocation (Variables|/Game/Blueprints/Components/Retaliation.Retaliation_C|GetCurrentAggressor (Variables|Default|GetRetaliation))))))

(fn FaceCourse
  (bind _returnvalue (Pawn|GetControlledPawn))
  (bind _velocity (Class|HasVelocity|Velocity(Message) _returnvalue))
  (Pawn|SetControlRotation (Math|Rotator|MakeRotfromXZ _velocity (Transformation|GetActorUpVector _returnvalue))))