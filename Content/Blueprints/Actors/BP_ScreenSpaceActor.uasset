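; Actor that stays pinned to a screen position in the 3D world, following the view of a given player controller.
; Each tick it scales its relative screen position by viewport size, deprojects it to world space, and pushes it along the view ray by an offset.
; It also copies the player camera's rotation.
; The actor destroys itself when the player controller is no longer valid.
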(event EventBeginPlay)

(event Collision|EventActorBeginOverlap
  (params (OtherActor :type Actor%20Object%20Reference)))

(event EventTick
  (params (DeltaSeconds :type Float%20%28single-precision%29))
  (Utilities|IsValid (Variables|Default|GetPlayerController)
    (:Is%20Valid
      (Transformation|SetActorLocationAndRotation (CallFunction|ScreenPositioninWorldSpace) (CallFunction|PlayerCameraRotation)))
    (:Is%20Not%20Valid
      (Actor|DestroyActor))))

(fn ConstructionScript)

(fn ScreenPositioninWorldSpace
  (bind _returnvalue (Viewport|GetViewportSize))
  (bind _playercontroller (Variables|Default|GetPlayerController))
  (bind _screenposition (Variables|Default|GetScreenPosition))
  (bind _returnvalue_2 (* _returnvalue _screenposition))
  (bind (_worldposition _worlddirection) (Class|GameplayStatics|DeprojectScreentoWorld _playercontroller _returnvalue_2))
  (return (+ _worldposition (* _worlddirection (Variables|Default|GetDirectionOffset)))))

(fn PlayerCameraRotation
  (return (Camera|GetCameraRotation (Variables|/Script/Engine.PlayerController|GetPlayerCameraManager (Variables|Default|GetPlayerController)))))