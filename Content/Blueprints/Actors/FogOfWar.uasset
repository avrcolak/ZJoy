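; FogOfWar is an actor that displays a fog of war material on a plane, shaped by two ellipse semi-axis lengths.
; The construction script creates a dynamic instance of that material on the plane, then applies the stored axis lengths.
; SetAxesLengths stores new lengths and writes them to the material's X and Y semi-axis scalar parameters.
; The event graph contains only disabled default events.
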(event EventBeginPlay
  (|CallParentFunction) ; This node is disabled and will not be called.\nDrag off pins to build functionality.
)

(event Collision|EventActorBeginOverlap
  (params (OtherActor :type Actor%20Object%20Reference))
  (|CallParentFunction OtherActor) ; This node is disabled and will not be called.\nDrag off pins to build functionality.
)

(event EventTick
  (params (DeltaSeconds :type Float%20%28single-precision%29))
  (|CallParentFunction DeltaSeconds) ; This node is disabled and will not be called.\nDrag off pins to build functionality.
)

(fn ConstructionScript
  (|CallParentFunction)
  (bind _returnvalue (Rendering|Material|CreateDynamicMaterialInstance (Variables|Default|GetPlane) 0 "/Game/Materials/FogOfWar.FogOfWar" "None" :!class /Script/Engine.PrimitiveComponent))
  (Variables|Default|SetFogOfWar _returnvalue)
  (CallFunction|SetAxesLengths (Variables|Default|GetAxesLengths)))

(fn SetAxesLengths
  (params (AxesLengths :type Vector%202D%20Structure))
  (bind _fogofwar (Variables|Default|GetFogOfWar))
  (bind _output_get (Variables|Default|SetAxesLengths AxesLengths))
  (Rendering|Material|SetScalarParameterValue _fogofwar "SemiAxisLengthX" (.X (Math|Vector2D|BreakVector2D _output_get)) :!class /Script/Engine.MaterialInstanceDynamic)
  (Rendering|Material|SetScalarParameterValue _fogofwar "SemiAxisLengthY" (.Y (Math|Vector2D|BreakVector2D _output_get)) :!class /Script/Engine.MaterialInstanceDynamic))