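; Arena actor that stages a sequencer-driven fight against spawned adversaries while a contestant stands in its trigger.
; Entry plays or resumes a spawned BP_ArenaSequence, re-orienting its origin opposite the contestant's forward vector when no adversaries remain.
; Play rate drives pacing: normal as adversaries join, fast-forward once cleared, and delayed rewind after the contestant leaves and adversaries are killed.
; Reinforce spawns controller-possessed phantoms; Die fades the circle's glow before destruction.
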(event OnComponentBeginOverlap(Trigger)
  (params (OverlappedComponent :type Primitive%20Component%20Object%20Reference) (OtherActor :type Actor%20Object%20Reference) (OtherComp :type Primitive%20Component%20Object%20Reference) (OtherBodyIndex :type Integer) (bFromSweep :type Boolean) (SweepResult :type Hit%20Result%20Structure%20%28by%20ref%29))
  (Variables|Default|SetContestant OtherActor)
  (Utilities|FlowControl|Sequence
    (:then_0
      (Utilities|When (CallFunction|NoAdversaries))
      (CallFunction|ResetSequenceTransformOrigin))
    (:then_1
      (Utilities|IsValid (Variables|Default|GetSequencePlayer)
        (:Is%20Valid
          (if (CallFunction|NoAdversaries)
            (CallFunction|RestartSequencePlayback)
            (else
              (Variables|Default|SetPendingRestartPlayback true))))
        (:Is%20Not%20Valid
          (bind _sequenceplayer (CallFunction|LoadSequence))
          (bind _output_get (Variables|Default|SetSequencePlayer _sequenceplayer))
          (Sequencer|Player|Play _output_get :!class /Script/MovieScene.MovieSceneSequencePlayer))))))

(event OnComponentEndOverlap(Trigger)
  (params (OverlappedComponent :type Primitive%20Component%20Object%20Reference) (OtherActor :type Actor%20Object%20Reference) (OtherComp :type Primitive%20Component%20Object%20Reference) (OtherBodyIndex :type Integer))
  (Variables|Default|SetContestant 0)
  (bind _arrayelement (Utilities|Array|ReverseforEachLoop (Variables|Default|GetAdversaries))
    (:LoopBody
      (Class|BPIDies|Die(Message) _arrayelement))
    (:Completed
      (Components|Timeline|SetPlayRate (Variables|Default|GetSequencePlayer) 0.0)
      (bind _returnvalue (Utilities|Time|SetTimerbyEvent (delegate Custom|ReversePlayback) 1.0))
      (Variables|Default|SetReversePlaybackDelay _returnvalue))))

(event Custom|ReversePlayback
  (Components|Timeline|SetPlayRate (Variables|Default|GetSequencePlayer) -3.0))

(event Custom|AddAdversary
  (params (Adversary :type BP%20Phantom%20Base%20Object%20Reference))
  (Utilities|Array|Add (Variables|Default|GetAdversaries) Adversary)
  (Game|BindEventtoOnDestroyed Adversary (delegate Custom|RemoveAdversary))
  (Components|Timeline|SetPlayRate (Variables|Default|GetSequencePlayer) 1.0))

(event Custom|RemoveAdversary
  (params (DestroyedActor :type Actor%20Object%20Reference))
  (Utilities|Array|RemoveItem (Variables|Default|GetAdversaries) DestroyedActor)
  (Utilities|IsValid (Variables|Default|GetContestant)
    (:Is%20Valid
      (Utilities|When (CallFunction|NoAdversaries))
      (Components|Timeline|SetPlayRate (Variables|Default|GetSequencePlayer) 3.0)
      (Default|CallOnAllAdversariesDestroyed))))

(event Custom|RestartPlaybackWhenPending
  (Utilities|When (Variables|Default|GetPendingRestartPlayback))
  (CallFunction|RestartSequencePlayback))

(event EventBeginPlay
  (bind _returnvalue (Game|SpawnActorfromClass "/Game/Blueprints/Actors/BP_ArenaSequence.BP_ArenaSequence_C" (CallFunction|UnitTransform) "Undefined" 0 self 0))
  (Variables|Default|SetSequence _returnvalue)
  (EventDispatchers|BindEventtoOnAllAdversariesDestroyed (delegate Custom|RestartPlaybackWhenPending)))

(event EventDie
  (Collision|SetCollisionEnabled (Variables|Default|GetTrigger) "NoCollision")
  (bind _emissivestrength (Timeline|Fade Play)
    (:Update
      (Rendering|Material|SetScalarParameterValue (Variables|Default|GetCircleMaterial) "EmissiveStrength" _emissivestrength :!class /Script/Engine.MaterialInstanceDynamic))
    (:Finished
      (Actor|DestroyActor))))

(fn ConstructionScript
  (bind _returnvalue (Rendering|Material|CreateDynamicMaterialInstance (Variables|Default|GetCircle) 0 0 "None" :!class /Script/Engine.PrimitiveComponent))
  (Variables|Default|SetCircleMaterial _returnvalue))

(fn LoadSequence
  (bind _sequence (Variables|Default|GetSequence))
  (bind _sequence_2 (Variables|Default|GetSequence))
  (bind _sequenceplayer (Variables|/Script/LevelSequence.LevelSequenceActor|GetSequencePlayer _sequence_2))
  (Class|LevelSequenceActor|SetSequence (Variables|Default|GetSequence) "/Game/Sequences/LS_PlaceHolder.LS_PlaceHolder")
  (Class|LevelSequenceActor|AddBinding _sequence (|GetSequenceBinding) _sequence false)
  (EventDispatchers|BindEventtoOnFinished _sequenceplayer (EventDispatchers|CreateEvent :!event Die))
  (return _sequenceplayer))

(fn ResetSequenceTransformOrigin
  (Default|SetTransformOrigin (Variables|Default|GetSequence) (Math|Transform|MakeTransform (Transformation|GetActorLocation) (Math|Rotator|MakeRotfromX (* (Transformation|GetActorForwardVector (Variables|Default|GetContestant)) -1.0)) "1,1,1")))

(fn NoAdversaries
  (return (<= (Utilities|Array|Length (Variables|Default|GetAdversaries)) 0)))

(fn RestartSequencePlayback
  (bind _sequenceplayer (Variables|Default|GetSequencePlayer))
  (Utilities|Time|ClearandInvalidateTimerbyHandle (Variables|Default|GetReversePlaybackDelay))
  (Components|Timeline|SetPlayRate _sequenceplayer 1.0)
  (Class|MovieSceneSequencePlayer|ScrubtoFrame _sequenceplayer (Utilities|Struct|MakeFrameTime (Utilities|Struct|MakeFrameNumber (Math|Integer|Max(Integer) (CallFunction|GetCurrentFrame _sequenceplayer))) 0.0)))

(fn CenterOfAttraction
  (return (Transformation|GetActorLocation)))

(fn NumberOfLives
  (return 0))

(fn Reinforce
  (bind _returnvalue (Game|SpawnActorfromClass "/Game/Blueprints/Actors/BP_SmallPhantom.BP_SmallPhantom_C" (CallFunction|UnitTransform) "Undefined" 0 0))
  (bind _output_get (LocalVariables|SetPhantom _returnvalue))
  (CallFunction|AddAdversary _output_get)
  (bind _returnvalue_2 (Game|SpawnActorfromClass "/Game/Blueprints/Actors/BP_FaceNearbyHero.BP_FaceNearbyHero_C" (CallFunction|UnitTransform) "Undefined" 0 0))
  (Class|Possesses|PossessQuickandDirty _returnvalue_2 (LocalVariables|GetPhantom))
  (return (LocalVariables|GetPhantom)))