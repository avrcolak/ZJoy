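; Player hero ship that moves by input, fires bullets on a looping timer, and cycles a speed multiplier shown by mesh scale.
; Each living tick moves it and offsets the spring arm toward its facing along an aspect-ratio-adjusted ellipse.
; Overlapping AttractsCamera actors pin the camera to their center until overlap ends.
; Hits cost a life, fading the ship, then destroying it or respawning it through flash timelines with temporarily relaxed collision.
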(event OnComponentBeginOverlap(HitBox)
  (params (OverlappedComponent :type Primitive%20Component%20Object%20Reference) (OtherActor :type Actor%20Object%20Reference) (OtherComp :type Primitive%20Component%20Object%20Reference) (OtherBodyIndex :type Integer) (bFromSweep :type Boolean) (SweepResult :type Hit%20Result%20Structure%20%28by%20ref%29))
  (bind _asattracts_camera (Utilities|Casting|CastToAttractsCamera OtherActor))
  (bind _output_get (Variables|Default|SetAttractor _asattracts_camera))
  (CallFunction|SnapCameratoAttractor _output_get))

(event OnComponentEndOverlap(HitBox)
  (params (OverlappedComponent :type Primitive%20Component%20Object%20Reference) (OtherActor :type Actor%20Object%20Reference) (OtherComp :type Primitive%20Component%20Object%20Reference) (OtherBodyIndex :type Integer))
  (Utilities|When (== OtherActor (Utilities|ToObject(Interface) (Variables|Default|GetAttractor))))
  (CallFunction|FreeCamera))

(event OnComponentHit(HitBox)
  (params (HitComponent :type Primitive%20Component%20Object%20Reference) (OtherActor :type Actor%20Object%20Reference) (OtherComp :type Primitive%20Component%20Object%20Reference) (NormalImpulse :type Vector :default "0, 0, 0") (Hit :type Hit%20Result%20Structure%20%28by%20ref%29))
  (Utilities|WhenAlive)
  (CallFunction|Die))

(event Custom|Shoot
  (Utilities|WhenAlive)
  (CallFunction|SpawnBullet))

(event Custom|StartShooting
  (bind _returnvalue (Utilities|Time|SetTimerbyEvent (delegate Custom|Shoot) 0.1667 true))
  (CallFunction|Shoot))

(event Custom|StopShooting
  (Utilities|Time|ClearandInvalidateTimerbyHandle (stale Custom|StartShooting _returnvalue)))

(event Custom|ServerSpawnBullet
  (CallFunction|SpawnBullet))

(event EventDie
  (Gameplay|Die))

(event EventTick
  (params (DeltaSeconds :type Float%20%28single-precision%29))
  (Utilities|WhenAlive)
  (CallFunction|Move DeltaSeconds)
  (CallFunction|AdjustSpringArm))

(event EventCycleSpeedMultiplier
  (Utilities|WhenAlive)
  (Math|Float|DecrementFloat (Variables|Default|GetSpeedMultiplier)
    (:%20%20
      (if (<= (Variables|Default|GetSpeedMultiplier) 1.0)
        (Variables|Default|SetSpeedMultiplier 4.0))
      (CallFunction|UpdateSpeedMultiplierMesh (Variables|Default|GetSpeedMultiplier)))))

(fn ConstructionScript
  (Variables|Default|SetInitialDistanceBetweenHullAndSpringArm (Math|Vector|Distance2D(Vector) (Transformation|GetWorldLocation (Variables|Default|GetSpringArm)) (Transformation|GetWorldLocation (Variables|Default|GetHull))))
  (Variables|Default|SetInitialSpeedMultiplierMeshScaleZ (.z (Transformation|GetWorldScale (Variables|Default|GetSpeedMutiplierMesh))))
  (bind _returnvalue (Rendering|Material|CreateDynamicMaterialInstance (Variables|Default|GetHull) 0 0 "None" :!class /Script/Engine.PrimitiveComponent))
  (Variables|Materials|SetHullMaterial _returnvalue)
  (bind _returnvalue_2 (Rendering|Material|CreateDynamicMaterialInstance (Variables|Default|GetSpeedMutiplierMesh) 0 0 "None" :!class /Script/Engine.PrimitiveComponent))
  (Variables|Materials|SetSpeedMultiplierMeshMaterial _returnvalue_2)
  (bind _returnvalue_3 (Rendering|Material|CreateDynamicMaterialInstance (Variables|Default|GetHitBoxMesh) 0 0 "None" :!class /Script/Engine.PrimitiveComponent))
  (Variables|Materials|SetHitBoxMeshMaterial _returnvalue_3)
  (CallFunction|UpdateSpeedMultiplierMesh (Variables|Default|GetSpeedMultiplier)))

(fn SpringArmDistancewhenFacing
  (params (Point :type Vector%202D%20Structure))
  (bind _initialdistancebetweenhullandspringarm (Variables|Default|GetInitialDistanceBetweenHullAndSpringArm))
  (bind _semiaxeslengths (CallFunction|SemiAxesLengthsatViewportAspectRatio _initialdistancebetweenhullandspringarm))
  (bind (_x _y) (Math|Vector2D|BreakVector2D _semiaxeslengths))
  (return (* (Math|Float|Clamp(Float) (Math|Float|Square (Variables|Default|GetFacingInputMagnitude))) (Math|Vector2D|Vector2DLength (Class|ZJoyBlueprintFunctionLibrary|EllipseLineIntersection Point _x _y)))))

(fn SpawnBullet
  (bind _returnvalue (Transformation|GetActorRotation))
  (Game|SpawnActorfromClass "/Game/Blueprints/Actors/HeroBullet.HeroBullet_C" (Math|Transform|MakeTransform (+ (Transformation|GetActorLocation) (Math|Vector|RotateVector "100.000000, 0, 0" _returnvalue)) _returnvalue) "Undefined" 0 self))

(fn MatchSpringArmLocationtoFacingVector
  (params (Point :type Vector))
  (bind _returnvalue (CallFunction|RotateWorldtoCamera Point))
  (Transformation|SetRelativeLocation (Variables|Default|GetSpringArm) (Math|Vector|MakeVector (CallFunction|SpringArmDistancewhenFacing (Math|Vector2D|MakeVector2D (.y _returnvalue) (.z _returnvalue))) 0.0 0.0) false false))

(fn Move
  (params (DeltaSeconds :type Float%20%28single-precision%29))
  (bind _returnvalue (Class|Pawn|ConsumeMovementInputVector))
  (Variables|Default|SetCurrentVelocity (* (Math|Vector|ClampVectorSize _returnvalue 0.0 1.0) (* (Variables|Default|GetSpeed) (Variables|Default|GetSpeedMultiplier))))
  (Transformation|SetActorLocationAndRotation (+ (* (* (Math|Vector|ClampVectorSize _returnvalue 0.0 1.0) (* (Variables|Default|GetSpeed) (Variables|Default|GetSpeedMultiplier))) DeltaSeconds) (Transformation|GetActorLocation)) (Pawn|GetControlRotation :!class /Script/Engine.Pawn) true))

(fn SemiAxesLengthsatViewportAspectRatio
  (params (UnitRadius :type Float%20%28single-precision%29))
  (bind _aspectratio (CallFunction|GetViewportAspectRatio))
  (return (Math|Vector2D|MakeVector2D (* (Math|Float|Clamp(Float) _aspectratio 1.0 1.33) UnitRadius) (* (Math|Float|Clamp(Float) (/ 1.0 _aspectratio) 1.0 1.33) UnitRadius))))

(fn AdjustSpringArm
  (Utilities|Unless (Variables|/Script/Engine.SceneComponent|GetbAbsoluteLocation (Variables|Default|GetSpringArm)))
  (CallFunction|MatchSpringArmLocationtoFacingVector (Transformation|GetActorForwardVector)))

(fn RotateWorldtoCamera
  (params (A :type Vector))
  (return (Math|Vector|RotateVector A (Class|KismetMathLibrary|NegateRotator (Transformation|GetWorldRotation (Variables|Default|GetCamera))))))

(fn SetModelOpacity
  (params (Opacity :type Float%20%28single-precision%29))
  (Rendering|Material|SetScalarParameterValue (Variables|Materials|GetHullMaterial) "Opacity" Opacity :!class /Script/Engine.MaterialInstanceDynamic)
  (Rendering|Material|SetScalarParameterValue (Variables|Materials|GetSpeedMultiplierMeshMaterial) "Opacity" Opacity :!class /Script/Engine.MaterialInstanceDynamic)
  (Rendering|Material|SetScalarParameterValue (Variables|Materials|GetHitBoxMeshMaterial) "Opacity" Opacity :!class /Script/Engine.MaterialInstanceDynamic))

(fn SnapCameratoAttractor
  (params (Attractor :type Attracts%20Camera%20Interface))
  (bind _centerofattraction (Default|CenterOfAttraction Attractor))
  (Utilities|FlowControl|Sequence
    (:then_0
      (Variables|/Script/Engine.SceneComponent|SetbAbsoluteLocation (Variables|Default|GetSpringArm) true))
    (:then_1
      (Transformation|SetWorldLocation (Variables|Default|GetSpringArm) _centerofattraction false false))))

(fn FreeCamera
  (Variables|/Script/Engine.SceneComponent|SetbAbsoluteLocation (Variables|Default|GetSpringArm) false))

(fn UpdateSpeedMultiplierMesh
  (params (Multiplier :type Float%20%28single-precision%29))
  (bind _speedmutipliermesh (Variables|Default|GetSpeedMutiplierMesh))
  (bind _returnvalue (Transformation|GetWorldScale _speedmutipliermesh))
  (Transformation|SetWorldScale3D _speedmutipliermesh (Math|Vector|MakeVector (.x _returnvalue) (.y _returnvalue) (* Multiplier (Variables|Default|GetInitialSpeedMultiplierMeshScaleZ)))))

(fn NumberOfLives
  (return (Variables|Default|GetLives)))