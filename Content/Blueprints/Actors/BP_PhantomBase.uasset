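; BP_PhantomBase is a base actor for phantom enemies that fire BP_PhantomBullet projectiles and carry a score worth.
; A HitBox overlap or hit while alive disables collision, fires OnDeath and fades the dynamic hull material through a timeline before destroying the actor.
; Helpers spawn bullets along the actor's transform, at given yaws, or in a randomly rotated three-petal flower built by splitting arcs into zero-width angles at stepped speeds.
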(event OnComponentHit(HitBox)
  (params (HitComponent :type Primitive%20Component%20Object%20Reference) (OtherActor :type Actor%20Object%20Reference) (OtherComp :type Primitive%20Component%20Object%20Reference) (NormalImpulse :type Vector :default "0, 0, 0") (Hit :type Hit%20Result%20Structure%20%28by%20ref%29))
  (Utilities|WhenAlive)
  (CallFunction|Die))

(event OnComponentBeginOverlap(HitBox)
  (params (OverlappedComponent :type Primitive%20Component%20Object%20Reference) (OtherActor :type Actor%20Object%20Reference) (OtherComp :type Primitive%20Component%20Object%20Reference) (OtherBodyIndex :type Integer) (bFromSweep :type Boolean) (SweepResult :type Hit%20Result%20Structure%20%28by%20ref%29))
  (Utilities|WhenAlive)
  (CallFunction|Die))

(event EventDie
  (Variables|Default|SetAlive false)
  (Collision|SetActorEnableCollision false)
  (Default|CallOnDeath self)
  (bind _opacity (Timeline|Fade Play)
    (:Update
      (Variables|Default|SetHullOpacity _opacity))
    (:Finished
      (Actor|DestroyActor))))

(event EventTick
  (params (DeltaSeconds :type Float%20%28single-precision%29))
  (Rendering|Material|SetScalarParameterValue (Variables|Default|GetHullMaterial) "Opacity" (Variables|Default|GetHullOpacity) :!class /Script/Engine.MaterialInstanceDynamic))

(fn ConstructionScript
  (bind _returnvalue (Rendering|Material|CreateDynamicMaterialInstance (Variables|Default|GetHull) 0 0 "None" :!class /Script/Engine.PrimitiveComponent))
  (Variables|Default|SetHullMaterial _returnvalue))

(fn SpawnBulletsatDegenerateArcs
  (params (Array :type Array%20of%20Vector%202D%20Structures) (InitialSpeed :type Float%20%28single-precision%29))
  (for _array_element Array
    (CallFunction|SpawnBulletatYaw InitialSpeed (.X (Math|Vector2D|BreakVector2D _array_element)))))

(fn SpawnBulletsinThreePointFlowerPattern
  (bind _output_get (LocalVariables|SetRandomOffset (Math|Random|RandomFloatinRange 0.0 1.2e+02)))
  (for _array_element (Class|ZJoyBlueprintFunctionLibrary|SplitArc "(X=0.000000,Y=360.000000)" 3 6e+01)
    (CallFunction|SpawnBulletsatDegenerateArcs (Class|ZJoyBlueprintFunctionLibrary|SplitArc (+ _array_element _output_get) 1 0.0) 1e+03)
    (CallFunction|SpawnBulletsatDegenerateArcs (Class|ZJoyBlueprintFunctionLibrary|SplitArc (+ _array_element _output_get) 2 0.0) 8e+02)
    (CallFunction|SpawnBulletsatDegenerateArcs (Class|ZJoyBlueprintFunctionLibrary|SplitArc (+ _array_element _output_get) 3 0.0) 6e+02)
    (CallFunction|SpawnBulletsatDegenerateArcs (Class|ZJoyBlueprintFunctionLibrary|SplitArc (+ _array_element _output_get) 4 0.0) 4e+02)))

(fn SpawnBulletatYaw
  (params (InitialSpeed :type Float%20%28single-precision%29) (Yaw :type Float%20%28single-precision%29))
  (Game|SpawnActorfromClass "/Game/Blueprints/Actors/BP_PhantomBullet.BP_PhantomBullet_C" (Math|Transform|MakeTransform (Transformation|GetActorLocation) (Math|Rotator|MakeRotator 0.0 0.0 Yaw)) "Undefined" 0 InitialSpeed self))

(fn SpawnBullet
  (params (InitialSpeed :type Float%20%28single-precision%29))
  (Game|SpawnActorfromClass "/Game/Blueprints/Actors/BP_PhantomBullet.BP_PhantomBullet_C" (Transformation|GetActorTransform) "Undefined" 0 InitialSpeed self))

(fn NumberOfLives
  (return 0))

(fn Worth
  (return (Variables|Default|GetScoreWorth)))