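; EnemyBullet is an enemy projectile that fades, slows and breaks apart near the end of its lifespan.
; Construction sets the launch speed and a dynamic material for emissive glow.
; A timer firing DestructionLength before lifespan expiry disables collision and plays the SpeedDecay timeline, scaling glow and compounding velocity decay each update.
; When the timeline finishes, radius damage at a randomly offset point fractures the bullet's own destructible component.
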(event Custom|Destruct
  (bind _projectilemovement (Variables|Default|GetProjectileMovement))
  (Collision|SetCollisionEnabled (Variables|Default|GetBullet) "NoCollision")
  (bind _1_decay (Timeline|SpeedDecay Play)
    (:Update
      (CallFunction|SetEmissiveStrength (* (Variables|Default|GetInitialEmissiveStrength) _1_decay))
      (Variables|/Script/Engine.MovementComponent|SetVelocity _projectilemovement (* (Variables|/Script/Engine.MovementComponent|GetVelocity _projectilemovement) _1_decay)))
    (:Finished
      (Class|DestructibleComponent|ApplyRadiusDamage (Variables|Default|GetBullet) 2.0 (+ (Transformation|GetActorLocation) (* (Math|Random|RandomUnitVector) 1e+01)) 1e+02 1.0 true))))

(event EventBeginPlay
  (Utilities|Time|SetTimerbyEvent (delegate Custom|Destruct) (- (Variables|Actor|GetInitialLifeSpan) (Variables|Default|GetDestructionLength))))

(fn ConstructionScript
  (Variables|/Script/Engine.ProjectileMovementComponent|SetInitialSpeed (Variables|Default|GetProjectileMovement) (Variables|Default|GetInitialSpeed))
  (bind _returnvalue (Rendering|Material|CreateDynamicMaterialInstance (Variables|Default|GetBullet) 0 "/Game/Materials/EnemyBullet.EnemyBullet" "None" :!class /Script/Engine.PrimitiveComponent))
  (Variables|Default|SetBulletMaterial _returnvalue)
  (CallFunction|SetEmissiveStrength (Variables|Default|GetInitialEmissiveStrength)))

(fn SetEmissiveStrength
  (params (Value :type Float%20%28single-precision%29))
  (Rendering|Material|SetScalarParameterValue (Variables|Default|GetBulletMaterial) "EmissiveStrength" Value :!class /Script/Engine.MaterialInstanceDynamic))