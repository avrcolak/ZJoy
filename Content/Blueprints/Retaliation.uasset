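; Retaliation Blueprint that calls its OnRetaliate dispatcher at a set frequency while it has aggressors.
; IncrementAggressors counts up and, if no timer is active, starts a looping timer and attempts retaliation immediately.
; When the count drops to zero, DecrementAggressors only flags the timer, which TryRetaliate clears on its next tick.
; A new aggressor arriving before then cancels the pending clear, preserving the cadence without an extra immediate retaliation.
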(fn IncrementAggressors
  (if (Utilities|Time|IsTimerActivebyHandle (Variables|Default|GetRetaliationTimer))
    (Variables|Default|SetPendingRetaliationTimerClear false)
    (else
      (bind _returnvalue (Utilities|Time|SetTimerbyFunctionName 0 "TryRetaliate" (Variables|Default|GetFrequency) true))
      (Variables|Default|SetRetaliationTimer _returnvalue)
      (CallFunction|TryRetaliate)))
  (Math|Integer|IncrementInt (Variables|Default|GetAggressors)))

(fn DecrementAggressors
  (bind _result (Math|Integer|DecrementInt (Variables|Default|GetAggressors))
    (:%20%20
      (Utilities|When (<= _result 0))
      (Variables|Default|SetPendingRetaliationTimerClear true))))

(fn TryRetaliate
  (if (Variables|Default|GetPendingRetaliationTimerClear)
    (Utilities|Time|ClearandInvalidateTimerbyHandle (Variables|Default|GetRetaliationTimer))
    (Variables|Default|SetPendingRetaliationTimerClear false)
    (else
      (Default|CallOnRetaliate))))