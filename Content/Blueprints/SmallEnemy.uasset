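; SmallEnemy is an enemy pawn that glides toward a goal location and rotation and can fire bullets.
; While alive, Tick moves and turns it at constant interpolation speeds by setting the transform directly, without sweeping.
; Moveto and Rotateto events set those goals, and Shoot calls SpawnBullet with a fixed value.
; The pawn destroys itself when unpossessed.
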(event EventUnpossessed
  (params (OldController :type Controller%20Object%20Reference))
  (Actor|DestroyActor))

(event EventShoot
  (params (Target :type Vector :default "0, 0, 0"))
  (CallFunction|SpawnBullet 1.6e+03))

(event EventRotateto
  (params (Goal :type Rotator :default "0, 0, 0"))
  (Variables|Default|SetGoalRotation Goal))

(event EventMoveto
  (params (Goal :type Vector :default "0, 0, 0"))
  (Variables|Default|SetGoalLocation Goal))

(event EventTick
  (params (DeltaSeconds :type Float%20%28single-precision%29))
  (Utilities|When (Variables|Default|GetAlive))
  (Transformation|SetActorLocation (Math|Interpolation|VInterptoConstant (Transformation|GetActorLocation) (Variables|Default|GetGoalLocation) DeltaSeconds (Variables|Default|GetSpeed)) false false)
  (Transformation|SetActorRotation (Class|KismetMathLibrary|RInterptoConstant (Transformation|GetActorRotation) (Variables|Default|GetGoalRotation) (Utilities|Time|GetWorldDeltaSeconds) (Variables|Default|GetRotationSpeed))))

(fn ConstructionScript)