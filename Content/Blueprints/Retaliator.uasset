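; Retaliator Blueprint that fires a retaliate call at a fixed frequency while it has active aggressors.
; Incrementing the aggressor count starts a looping timer with an immediate first retaliation, or cancels a pending stop if the timer is running.
; When the count drops to zero, timer clearing waits until the next tick of that timer, so quick re-engagement keeps the existing cadence.
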(fn IncrementAggressors
  (if (Utilities|Time|IsTimerActivebyHandle (Variables|Default|GetRetaliationTimer))
    (Variables|Default|SetPendingRetaliationTimerClear false)
    (else
      (bind _returnvalue (Utilities|Time|SetTimerbyFunctionName 0 "TryRetaliate" (Variables|Default|GetFrequency) true))
      (Variables|Default|SetRetaliationTimer _returnvalue)
      (CallFunction|TryRetaliate)))
  (Math|Integer|IncrementInt (Variables|Default|GetAggressors)))

(fn DecrementAggressors
  (bind _result (Math|Integer|DecrementInt (Variables|Default|GetAggressors))
    (:%20%20
      (Utilities|When (<= _result 0))
      (Variables|Default|SetPendingRetaliationTimerClear true))))

(fn TryRetaliate
  (if (Variables|Default|GetPendingRetaliationTimerClear)
    (Utilities|Time|ClearandInvalidateTimerbyHandle (Variables|Default|GetRetaliationTimer))
    (Variables|Default|SetPendingRetaliationTimerClear false)
    (else
      (Default|CallOnRetaliate))))