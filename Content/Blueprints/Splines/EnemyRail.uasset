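; EnemyRail is a spline-folder Blueprint actor that moves itself toward a tracked component and serves as a rail for following actors.
; Each Tick, while TrackedComponent is valid, it uses a Move helper with Speed and delta time to step its location toward that component without sweeping.
; AddActor and RemoveActor keep a count of followers, and the rail destroys itself when a removal brings the count to zero or below.
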(event EventTick
  (params (DeltaSeconds :type Float%20%28single-precision%29))
  (bind _trackedcomponent (Variables|Default|GetTrackedComponent))
  (Utilities|IsValid _trackedcomponent
    (:Is%20Valid
      (Transformation|SetActorLocation (.NewLocation (CallFunction|Move (Transformation|GetWorldLocation _trackedcomponent) (Transformation|GetActorLocation) (Variables|Components|GetSpeed) (Utilities|Time|GetWorldDeltaSeconds))) false false))))

(fn ConstructionScript
  (|CallParentFunction))

(fn AddActor
  (Math|Integer|IncrementInt (Variables|Default|GetFollowingActors)))

(fn RemoveActor
  (bind _result (Math|Integer|DecrementInt (Variables|Default|GetFollowingActors))
    (:%20%20
      (Utilities|When (<= _result 0))
      (Actor|DestroyActor))))