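; Player ship pawn with twin-stick controls that moves along world X/Y and fires PawnShipBullet on a looping timer while Shoot is held.
; Each tick it applies swept movement and rotates toward facing input, falling back to last movement input, then current forward.
; The spring arm slides along ship forward to an aspect-weighted ellipse sized from its constructed offset, while MaintainMinorAxisFov updates the view.
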(event Custom|Shoot
  (CallFunction|SpawnBullet))

(event EventBeginPlay
  (Class|ZJoyBlueprintFunctionLibrary|MaintainMinorAxisFov self))

(event Collision|EventActorBeginOverlap
  (params (OtherActor :type Actor%20Object%20Reference)))

(event EventTick
  (params (DeltaSeconds :type Float%20%28single-precision%29))
  (bind _facingvector (CallFunction|GetFacingVector))
  (CallFunction|MoveForward DeltaSeconds)
  (Transformation|SetActorRotation (Math|Rotator|FindLookatRotation (Math|Vector|MakeVector 0.0 0.0 0.0) _facingvector))
  (CallFunction|MatchSpringArmLocationtoFacingVector (Math|Conversions|ToVector2D(Vector) _facingvector))
  (Class|ZJoyBlueprintFunctionLibrary|MaintainMinorAxisFov self))

(event Input|ActionEvents|InputActionShoot
  (params (Key :type Key%20Structure))
  (:Pressed
    (bind _returnvalue (Utilities|Time|SetTimerbyEvent (delegate Custom|Shoot) 0.1667 true)))
  (:Released
    (Utilities|Time|ClearandInvalidateTimerbyHandle _returnvalue)))

(event Input|AxisEvents|InputAxisMoveUp
  (params (AxisValue :type Float%20%28single-precision%29))
  (Pawn|Input|AddMovementInput "0.000000,1.000000,0.000000" AxisValue false))

(event Input|AxisEvents|InputAxisMoveRight
  (params (AxisValue :type Float%20%28single-precision%29))
  (Pawn|Input|AddMovementInput "1.000000,0.000000,0.000000" AxisValue false))

(event Input|AxisEvents|InputAxisFaceUp
  (params (AxisValue :type Float%20%28single-precision%29))
  (CallFunction|SetFacingY AxisValue))

(event Input|AxisEvents|InputAxisFaceRight
  (params (AxisValue :type Float%20%28single-precision%29))
  (CallFunction|SetFacingX AxisValue))

(fn ConstructionScript
  (Variables|Default|SetConstructedDistanceBetweenShipAndSpringArm (Math|Vector|Distance2D(Vector) (Transformation|GetWorldLocation (Variables|Default|GetSpringArm)) (Transformation|GetWorldLocation (Variables|Default|GetShip))))
  (Variables|Default|SetConstructedSpringArmLength (Variables|/Script/Engine.SpringArmComponent|GetTargetArmLength (Variables|Default|GetSpringArm))))

(fn SetFacingX
  (params (X :type Float%20%28single-precision%29))
  (Variables|Default|SetFacingInput (Math|Vector2D|MakeVector2D X (.Y (Math|Vector2D|BreakVector2D (Variables|Default|GetFacingInput))))))

(fn SetFacingY
  (params (Y :type Float%20%28single-precision%29))
  (Variables|Default|SetFacingInput (Math|Vector2D|MakeVector2D (.X (Math|Vector2D|BreakVector2D (Variables|Default|GetFacingInput))) Y)))

(fn SpringArmDistancewhenFacing
  (params (Point :type Vector%202D%20Structure))
  (bind _aspectratio (CallFunction|GetViewportAspectRatio))
  (bind _constructeddistancebetweenshipandspringarm (Variables|Default|GetConstructedDistanceBetweenShipAndSpringArm))
  (return (Math|Vector2D|Vector2DLength (Class|ZJoyBlueprintFunctionLibrary|EllipseLineIntersection Point (* _constructeddistancebetweenshipandspringarm (+ (* _aspectratio 0.5) 0.5)) (* _constructeddistancebetweenshipandspringarm (+ (/ 0.5 _aspectratio) 0.5))))))

(fn SpawnBullet
  (bind _returnvalue (Transformation|GetActorRotation))
  (Game|SpawnActorfromClass "/Game/Blueprints/PawnShipBullet.PawnShipBullet_C" (Math|Transform|MakeTransform (+ (Transformation|GetActorLocation) (Math|Vector|RotateVector "1.000000, 0, 0" _returnvalue)) _returnvalue) "Undefined" 0 0.0 0))

(fn MatchSpringArmLocationtoFacingVector
  (params (Point :type Vector%202D%20Structure))
  (Transformation|SetRelativeLocation (Variables|Default|GetSpringArm) (Math|Vector|MakeVector (CallFunction|SpringArmDistancewhenFacing Point) 0.0 0.0) false false))

(fn GetFacingVector
  (bind _returnvalue (Class|Pawn|GetLastMovementInputVector))
  (bind _facinginput (Variables|Default|GetFacingInput))
  (bind _returnvalue_2 (Class|KismetMathLibrary|IsNearlyZero2D _facinginput 0.0001))
  (bind _returnvalue_3 (Math|Conversions|ToVector(Vector2D) _facinginput))
  (bind _returnvalue_4 (select _returnvalue_2 _returnvalue _returnvalue_3))
  (return (select (Math|Vector|VectorIsNearlyZero _returnvalue_4) (Transformation|GetActorForwardVector) _returnvalue_4)))

(fn MoveForward
  (params (DeltaSeconds :type Float%20%28single-precision%29))
  (bind _returnvalue (Class|Pawn|ConsumeMovementInputVector))
  (Transformation|AddActorWorldOffset (* _returnvalue (* DeltaSeconds (Variables|Default|GetSpeed))) true))