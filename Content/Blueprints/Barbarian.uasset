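; Barbarian is an attacker actor that fires radial bullet patterns at nearby Pawns and destroys itself on any actor overlap.
; Tick sphere-checks for Pawns within AttackTriggerRadius, firing immediately and then on a looping timer until none remain.
; Each volley uses SplitArc to form three randomly rotated petals of BarbarianBullets.
; Each petal layers rows with more bullets at lower speeds, so the flower shape opens as they travel.
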(event Custom|AttackPawn
  (CallFunction|SpawnBulletsinThreePointFlowerPattern))

(event EventBeginPlay)

(event Collision|EventActorBeginOverlap
  (params (OtherActor :type Actor%20Object%20Reference))
  (Actor|DestroyActor))

(event EventTick
  (params (DeltaSeconds :type Float%20%28single-precision%29))
  (bind _returnvalue (Collision|SphereOverlapActors (Transformation|GetActorLocation) (Variables|Default|GetAttackTriggerRadius) (Utilities|Array|MakeArray "ObjectTypeQuery2") "/Game/Blueprints/Pawn.Pawn_C"))
  (if _returnvalue
    (if (not (Utilities|Time|IsTimerActivebyHandle (Variables|Default|GetTimer)))
      (CallFunction|AttackPawn)
      (bind _returnvalue_2 (Utilities|Time|SetTimerbyEvent (delegate Custom|AttackPawn) 5.0 true))
      (Variables|Default|SetTimer _returnvalue_2))
    (else
      (Utilities|Time|ClearandInvalidateTimerbyHandle (Variables|Default|GetTimer)))))

(fn ConstructionScript)

(fn SpawnBulletsatDegenerateArcs
  (params (Array :type Array%20of%20Vector%202D%20Structures) (InitialSpeed :type Float%20%28single-precision%29))
  (for _array_element Array
    (Game|SpawnActorfromClass "/Game/Blueprints/BarbarianBullet.BarbarianBullet_C" (Math|Transform|MakeTransform (Transformation|GetActorLocation) (Math|Rotator|MakeRotator 0.0 0.0 (.X (Math|Vector2D|BreakVector2D _array_element)))) "Undefined" 0 InitialSpeed 0)))

(fn SpawnBulletsinThreePointFlowerPattern
  (bind _output_get (LocalVariables|SetRandomOffset (Math|Random|RandomFloatinRange 0.0 1.2e+02)))
  (for _array_element (Class|ZJoyBlueprintFunctionLibrary|SplitArc "(X=0.000000,Y=360.000000)" 3 6e+01)
    (CallFunction|SpawnBulletsatDegenerateArcs (Class|ZJoyBlueprintFunctionLibrary|SplitArc (+ _array_element _output_get) 1 0.0) 1e+03)
    (CallFunction|SpawnBulletsatDegenerateArcs (Class|ZJoyBlueprintFunctionLibrary|SplitArc (+ _array_element _output_get) 2 0.0) 8e+02)
    (CallFunction|SpawnBulletsatDegenerateArcs (Class|ZJoyBlueprintFunctionLibrary|SplitArc (+ _array_element _output_get) 3 0.0) 6e+02)
    (CallFunction|SpawnBulletsatDegenerateArcs (Class|ZJoyBlueprintFunctionLibrary|SplitArc (+ _array_element _output_get) 4 0.0) 4e+02)))