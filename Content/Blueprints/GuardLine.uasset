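; GuardLine is a controller that makes its pawn guard a line around the controller's location, shadowing intruders.
; Player-controlled pawns overlapping GuardBox join an aggressor list; the first stays current until removed, then the next takes over.
; Each tick the pawn interpolates toward the aggressor's offset projected on the controller's axes, with forward distance halved.
; Without an aggressor, it eases back to the origin more slowly.
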(event OnComponentBeginOverlap(GuardBox)
  (params (OverlappedComponent :type Primitive%20Component%20Object%20Reference) (OtherActor :type Actor%20Object%20Reference) (OtherComp :type Primitive%20Component%20Object%20Reference) (OtherBodyIndex :type Integer) (bFromSweep :type Boolean) (SweepResult :type Hit%20Result%20Structure%20%28by%20ref%29))
  (bind _aspawn (Utilities|Casting|CastToPawn OtherActor))
  (Utilities|When (Pawn|IsPlayerControlled _aspawn))
  (CallFunction|AddAggressor _aspawn))

(event OnComponentEndOverlap(GuardBox)
  (params (OverlappedComponent :type Primitive%20Component%20Object%20Reference) (OtherActor :type Actor%20Object%20Reference) (OtherComp :type Primitive%20Component%20Object%20Reference) (OtherBodyIndex :type Integer))
  (CallFunction|RemoveAggressor OtherActor))

(event EventBeginPlay)

(event EventTick
  (params (DeltaSeconds :type Float%20%28single-precision%29))
  (Utilities|IsValid (Pawn|GetControlledPawn)
    (:Is%20Valid
      (Utilities|IsValid (Variables|Default|GetCurrentAggressor)
        (:Is%20Valid
          (CallFunction|MovePawnTowardsAggressor)
          (Rendering|Debug|DrawDebugPoint (Transformation|GetActorLocation (Variables|Default|GetCurrentAggressor)) 1e+01 "(R=1.000000,G=1.000000,B=0.000000,A=1.000000)" 0.0))
        (:Is%20Not%20Valid
          (CallFunction|MovePawnTowardsOrigin))))))

(event EventPossess
  (params (PossessedPawn :type Pawn%20Object%20Reference))
  (CallFunction|RemoveAggressor PossessedPawn))

(fn ConstructionScript)

(fn MovePawnTowardsAggressor
  (bind _returnvalue (Transformation|GetActorLocation))
  (bind _returnvalue_2 (Pawn|GetControlledPawn))
  (bind _currentaggressor (Variables|Default|GetCurrentAggressor))
  (bind _returnvalue_3 (Transformation|GetActorLocation _currentaggressor))
  (bind _returnvalue_4 (- _returnvalue_3 _returnvalue))
  (bind _asmoves (Utilities|Casting|CastToMoves _returnvalue_2))
  (Default|Moveto _asmoves (Math|Interpolation|VInterpTo (Transformation|GetActorLocation _returnvalue_2) (+ (Math|Vector|ProjectVectorontoVector _returnvalue_4 (Transformation|GetActorRightVector)) (* (Math|Vector|ProjectVectorontoVector _returnvalue_4 (Transformation|GetActorForwardVector)) 0.5) (Transformation|GetActorLocation)) (Utilities|Time|GetWorldDeltaSeconds) 3.0)))

(fn MovePawnTowardsOrigin
  (bind _returnvalue (Pawn|GetControlledPawn))
  (Class|Moves|Moveto(Message) _returnvalue (Math|Interpolation|VInterpTo (Transformation|GetActorLocation _returnvalue) (Transformation|GetActorLocation) (Utilities|Time|GetWorldDeltaSeconds) 0.5)))

(fn AddAggressor
  (params (Aggressor :type Actor%20Object%20Reference))
  (Utilities|Unless (== Aggressor (Pawn|GetControlledPawn)))
  (bind _returnvalue (Utilities|Array|Add (Variables|Default|GetAggressors) Aggressor))
  (Utilities|When (== _returnvalue 0))
  (Variables|Default|SetCurrentAggressor Aggressor))

(fn RemoveAggressor
  (params (Aggressor :type Actor%20Object%20Reference))
  (Utilities|Array|RemoveItem (Variables|Default|GetAggressors) Aggressor)
  (Utilities|When (== Aggressor (Variables|Default|GetCurrentAggressor)))
  (if (== (Utilities|Array|Length (Variables|Default|GetAggressors)) 0)
    (Variables|Default|SetCurrentAggressor 0)
    (else
      (Variables|Default|SetCurrentAggressor (Utilities|Array|Get(acopy) (Variables|Default|GetAggressors))))))