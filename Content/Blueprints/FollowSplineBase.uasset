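; Base controller that steers its possessed pawn along a spline, with optional aiming and shooting at a target.
; Each playback-position update samples the spline and sends move and rotate interface messages to the pawn.
; Rotation follows the spline plus an offset, or faces the target when look-at is toggled on and the target is valid.
; Shoot messages the pawn with the target's location, and the controller destroys itself on unpossess.
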(event EventUnPossess
  (params (UnpossessedPawn :type Pawn%20Object%20Reference))
  (Actor|DestroyActor))

(fn ConstructionScript)

(fn GoalRotation
  (params (Offset :type Rotator) (PlaybackPosition :type Float%20%28single-precision%29) (LookingAtTarget :type Boolean))
  (bind _returnvalue (CallFunction|CurrentRotationonSpline Offset PlaybackPosition))
  (Utilities|IsValid (Variables|Default|GetTarget)
    (:Is%20Valid
      (if LookingAtTarget
        (return (Math|Rotator|FindLookatRotation (Transformation|GetActorLocation (Pawn|GetControlledPawn)) (Transformation|GetActorLocation (Variables|Default|GetTarget))))
        (else
          (return _returnvalue))))
    (:Is%20Not%20Valid
      (return _returnvalue))))

(fn CurrentRotationonSpline
  (params (Offset :type Rotator) (PlaybackPosition :type Float%20%28single-precision%29))
  (return (Math|Rotator|CombineRotators (Class|SplineComponent|GetRotationatTime (Variables|Default|GetSpline) PlaybackPosition "World" false) Offset)))

(fn CurrentLocationonSpline
  (params (PlaybackPosition :type Float%20%28single-precision%29))
  (return (Spline|GetLocationatTime (Variables|Default|GetSpline) PlaybackPosition "World" false)))

(fn UpdatePlaybackPosition
  (params (PlaybackPosition :type Float%20%28single-precision%29) (Offset :type Rotator))
  (Class|Moves|Moveto(Message) (Pawn|GetControlledPawn) (CallFunction|CurrentLocationonSpline PlaybackPosition))
  (Class|Rotates|Rotateto(Message) (Pawn|GetControlledPawn) (CallFunction|GoalRotation Offset PlaybackPosition (Variables|Default|GetLookingAtTarget))))

(fn ToggleLookingatTarget
  (Variables|Default|SetLookingAtTarget (not (Variables|Default|GetLookingAtTarget))))

(fn Shoot
  (Class|Shoots|Shoot(Message) (Pawn|GetControlledPawn) (Transformation|GetActorLocation (Variables|Default|GetTarget))))